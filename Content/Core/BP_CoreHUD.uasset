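; Core HUD that owns the game's root UI widget stack and opens its screens.
; BeginPlay caches BP_GameInstance, then creates WBP_GameStack, adds it to the viewport and seeds its MainStack with the match overlay.
; One event per screen (main menu, options, match overlay, shop, transition, game setup, credits) calls PushWidget on the stack.
; Despite their Toggle names, these events only push and never close screens.
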(event `self.ReceiveBeginPlay`
  ;[1 1 1] On startup
  (`|ExecutionSequence`
    (:`then_0`
      (bind _asbp_game_instance (cast `/Game/Core/BP_GameInstance` (`GameplayStatics.GetGameInstance`)))
      (set `self.GameInstance` _asbp_game_instance))
    (:`then_1`
      (bind _returnvalue (`|CreateWidget` "/Game/Widget/WBP_GameStack.WBP_GameStack_C"))
      (bind _output_get (set `self.GameStack` _returnvalue))
      (`UserWidget.AddToViewport` _output_get 0)
      (`CommonActivatableWidgetContainerBase.BP_AddWidget` (`/Game/Widget/WBP_GameStack.MainStack` _output_get) "/Game/Widget/WBP_MatchOverlay.WBP_MatchOverlay_C"))))

(event `MainMenuToggle`
  (`/Game/Widget/WBP_GameStack.Push Widget` (`self.GameStack`) "/Game/Widget/WBP_MainMenu.WBP_MainMenu_C"))

(event `OptionsToggle`
  (`/Game/Widget/WBP_GameStack.Push Widget` (`self.GameStack`) "/Game/Widget/WBP_Options.WBP_Options_C"))

(event `MatchOverlayToggle`
  (`/Game/Widget/WBP_GameStack.Push Widget` (`self.GameStack`) "/Game/Widget/WBP_MatchOverlay.WBP_MatchOverlay_C"))

(event `ShopToggle`
  (`/Game/Widget/WBP_GameStack.Push Widget` (`self.GameStack`) "/Game/Widget/WBP_ShopInterface.WBP_ShopInterface_C"))

(event `TransitionToggle`
  (`/Game/Widget/WBP_GameStack.Push Widget` (`self.GameStack`) "/Game/Widget/WBP_Tansition.WBP_Tansition_C"))

(event `GameSettupToggle`
  (`/Game/Widget/WBP_GameStack.Push Widget` (`self.GameStack`) "/Game/Widget/WBP_GameSetup.WBP_GameSetup_C"))

(event `CreditToggle`
  (`/Game/Widget/WBP_GameStack.Push Widget` (`self.GameStack`) "/Game/Widget/WBP_Credits.WBP_Credits_C"))

(fn `UserConstructionScript`)