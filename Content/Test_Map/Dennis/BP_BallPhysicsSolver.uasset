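; BP_BallPhysicsSolver is a ball physics solver Blueprint that supplies exit direction and speed for ball-to-ball and ball-to-wall collisions.
; Separate functions cover the ball, the other ball and wall bounces, each receiving a suggested velocity plus hit context.
; All of them pass the suggestion through unchanged, returning its normalized vector as direction and its length as speed, ignoring the other inputs.
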(fn `BallCollisionSetExitDirection`
  (params (SuggestedVelocity :type "Vector Structure") (UnModifiedBall :type "BallActor Object Reference") (OtherBallActor :type "BallActor Object Reference") (Hit :type "HitResult Structure (by ref)"))
  (returns (ReturnValue :type "Vector Structure"))
  (return (`KismetMathLibrary.Normal` SuggestedVelocity)))

(fn `BallCollisionSetExitSpeed`
  (params (SuggestedVelocity :type "Vector Structure") (UnModifiedBall :type "BallActor Object Reference") (OtherBallActor :type "BallActor Object Reference") (OutDirection :type "Vector Structure") (Hit :type "HitResult Structure (by ref)"))
  (returns (ReturnValue :type "Float (single-precision)"))
  (return (`KismetMathLibrary.VSize` SuggestedVelocity)))

(fn `OtherBallCollisionSetExitDirection`
  (params (OtherBallSuggestedVelocity :type "Vector Structure") (OtherBallActor :type "BallActor Object Reference") (UnModifiedBall :type "BallActor Object Reference") (Hit :type "HitResult Structure (by ref)"))
  (returns (ReturnValue :type "Vector Structure"))
  (return (`KismetMathLibrary.Normal` OtherBallSuggestedVelocity)))

(fn `OtherBallCollisionSetExitSpeed`
  (params (OtherBallSuggestedVelocity :type "Vector Structure") (OtherBallActor :type "BallActor Object Reference") (UnModifiedBall :type "BallActor Object Reference") (OutDirection :type "Vector Structure") (Hit :type "HitResult Structure (by ref)"))
  (returns (ReturnValue :type "Float (single-precision)"))
  (return (`KismetMathLibrary.VSize` OtherBallSuggestedVelocity)))

(fn `WallCollisionSetExitDirection`
  (params (SuggestedVelocity :type "Vector Structure") (UnModifiedBall :type "BallActor Object Reference") (Hit :type "HitResult Structure (by ref)"))
  (returns (ReturnValue :type "Vector Structure"))
  (return (`KismetMathLibrary.Normal` SuggestedVelocity)))

(fn `WallCollisionSetExitSpeed`
  (params (SuggestedVelocity :type "Vector Structure") (UnModifiedBall :type "BallActor Object Reference") (Hit :type "HitResult Structure (by ref)"))
  (returns (ReturnValue :type "Float (single-precision)"))
  (return (`KismetMathLibrary.VSize` SuggestedVelocity)))