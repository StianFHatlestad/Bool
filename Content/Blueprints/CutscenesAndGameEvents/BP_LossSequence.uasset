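; BP_LossSequence is a loss cutscene actor that plays a table-shattering, vortex and void effect as soon as it begins play.
; It hides all BP_Table actors, then chains delayed Niagara crack and impact-frame effects with world camera shakes, and hides actors tagged HideOnLose.
; It then enables physics on ShatterableTable while a timeline drives ring, void and glow scalars in MPC_LossSequence, followed by a final break shake.
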(event `self.ReceiveBeginPlay`
  (`|ExecutionSequence`
    (:`then_0`
      (bind _outactors (`GameplayStatics.GetAllActorsOfClass` "/Game/Blueprints/Table/BP_Table.BP_Table_C"))
      (for _array_element _outactors
        (`self.SetActorHiddenInGame` _array_element true)))
    (:`then_1`
      (bind _returnvalue (`NiagaraFunctionLibrary.SpawnSystemAtLocation` "/Game/VFX/Niagara/Systems/Loss/NS_PreCrack.NS_PreCrack" (0.0 0.0 40.0)))
      (`GameplayStatics.PlayWorldCameraShake` "/Game/VFX/CameraShake/CS_LossCrackShake.CS_LossCrackShake_C" (`self.K2_GetActorLocation`) 0.0 20000.0 1.0 true)
      (`KismetSystemLibrary.Delay` 0.3)
      (`GameplayStatics.PlayWorldCameraShake` "/Game/VFX/CameraShake/CS_LossCrackShake.CS_LossCrackShake_C" (`self.K2_GetActorLocation`) 0.0 20000.0 1.0 true)
      (`KismetSystemLibrary.Delay` 0.5)
      (`ActorComponent.K2_DestroyComponent` _returnvalue)
      (`GameplayStatics.PlayWorldCameraShake` "/Game/VFX/CameraShake/CS_RedballBlastShake.CS_RedballBlastShake_C" (`self.K2_GetActorLocation`) 0.0 20000.0 1.0 true)
      (`NiagaraFunctionLibrary.SpawnSystemAtLocation` "/Game/VFX/Niagara/Systems/Loss/NS_Impactframe.NS_Impactframe" (0.0 0.0 96.02918))
      (`KismetSystemLibrary.Delay` 0.2)
      (bind _outactors_2 (`GameplayStatics.GetAllActorsWithTag` "HideOnLose"))
      (for _array_element_2 _outactors_2
        (`self.SetActorHiddenInGame` _array_element_2 true))
      (`|ExecutionSequence`
        (:`then_0`
          (`PrimitiveComponent.SetSimulatePhysics` (`self.ShatterableTable`) true))
        (:`then_1`
          (bind (_direction _vortexcurvescale _voidcurvescale _voidlightscale) (`Timeline|Timeline` :!via `PlayFromStart`)
            (:`Update`
              (`|ExecutionSequence`
                (:`then_0`
                  (`KismetMaterialLibrary.SetScalarParameterValue` "/Game/VFX/SequenceBased/Loss/MPC_LossSequence.MPC_LossSequence" "RingScale" (* _vortexcurvescale 1.170814)))
                (:`then_1`
                  (`KismetMaterialLibrary.SetScalarParameterValue` "/Game/VFX/SequenceBased/Loss/MPC_LossSequence.MPC_LossSequence" "VoidScale" (* _voidcurvescale 0.45)))
                (:`then_2`
                  (`KismetMaterialLibrary.SetScalarParameterValue` "/Game/VFX/SequenceBased/Loss/MPC_LossSequence.MPC_LossSequence" "TriGlow" (* _voidlightscale 22.0)))))))
        (:`then_2`
          (`KismetSystemLibrary.Delay` 0.3)
          (`GameplayStatics.PlayWorldCameraShake` "/Game/VFX/CameraShake/CS_LossBreakShake.CS_LossBreakShake_C" (`self.K2_GetActorLocation`) 0.0 20000.0 1.0 true))))))

(fn `UserConstructionScript`)