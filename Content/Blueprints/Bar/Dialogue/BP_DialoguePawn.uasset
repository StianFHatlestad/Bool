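; Bar dialogue pawn that offers an interaction prompt when the first-person player enters its box and can run a dialogue through its dialogue component.
; Overlap start toggles the HUD pop-up, focuses the pop-up stack in Game and UI input and sets InteractingInBar on the game instance.
; Overlap end removes the active pop-up, restores game-only input and clears the flag.
; RunDialogue forwards to the component; RunDialogueMessage is left unwired.
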(event `self.Box.OnComponentBeginOverlap`
  (params (OverlappedComponent :type "PrimitiveComponent Object Reference") (OtherActor :type "Actor Object Reference") (OtherComp :type "PrimitiveComponent Object Reference") (OtherBodyIndex :type Integer) (bFromSweep :type Boolean) (SweepResult :type "HitResult Structure (by ref)"))
  (bind _returnvalue (`GameplayStatics.GetPlayerController` 0))
  (cast `/Game/Blueprints/Core/BP_FirstPersonBool` OtherActor)
  (bind _asbp_core_hud (cast `/Game/Blueprints/Core/BP_CoreHUD` (`PlayerController.GetHUD` _returnvalue)))
  (`/Game/Blueprints/Core/BP_CoreHUD.Interaction PopUp Toggle` _asbp_core_hud)
  (`WidgetBlueprintLibrary.SetInputMode_GameAndUIEx` _returnvalue (`/Game/Widget/WBP_GameStack.PopUpStack` (`/Game/Blueprints/Core/BP_CoreHUD.GameStack` _asbp_core_hud)) "LockAlways")
  (bind _asbp_game_instance (cast `/Game/Blueprints/Core/BP_GameInstance` (`GameplayStatics.GetGameInstance`)))
  (set `/Game/Blueprints/Core/BP_GameInstance.InteractingInBar` true _asbp_game_instance))

(event `self.Box.OnComponentEndOverlap`
  (params (OverlappedComponent :type "PrimitiveComponent Object Reference") (OtherActor :type "Actor Object Reference") (OtherComp :type "PrimitiveComponent Object Reference") (OtherBodyIndex :type Integer))
  (bind _returnvalue (`GameplayStatics.GetPlayerController` 0))
  (cast `/Game/Blueprints/Core/BP_FirstPersonBool` OtherActor)
  (bind _asbp_core_hud (cast `/Game/Blueprints/Core/BP_CoreHUD` (`PlayerController.GetHUD` _returnvalue)))
  (bind _gamestack (`/Game/Blueprints/Core/BP_CoreHUD.GameStack` _asbp_core_hud))
  (`/Game/Widget/WBP_GameStack.Remove Pop up` _gamestack (`CommonActivatableWidgetContainerBase.GetActiveWidget` (`/Game/Widget/WBP_GameStack.PopUpStack` _gamestack)))
  (`WidgetBlueprintLibrary.SetInputMode_GameOnly` _returnvalue)
  (bind _asbp_game_instance (cast `/Game/Blueprints/Core/BP_GameInstance` (`GameplayStatics.GetGameInstance`)))
  (set `/Game/Blueprints/Core/BP_GameInstance.InteractingInBar` false _asbp_game_instance))

(fn `GetDialogueComponent`
  (returns (DialogueComponent :type "/Game/Blueprints/Bar/Dialogue/BP_DialogueComponent Object Reference"))
  (return null))

(fn `RunDialogue`
  (returns (Sucsess :type Boolean))
  (`/Game/Blueprints/Bar/Dialogue/BP_DialogueComponent.RunDialogue` (`self.BP_DialogueComponent`))
  (return false))

(fn `UserConstructionScript`)