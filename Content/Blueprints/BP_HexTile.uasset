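; Hex tile actor that reacts to mouse hover by lifting itself.
; When the cursor enters its sphere collider, it stores the current location and a slightly raised target, then a timeline lerps the actor upward.
; An end-cursor-over event plays a second timeline meant to lower it, but that lerp's alpha is fixed at zero, so it sets the tile to the raised position.
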(event `self.SphereCollider.OnBeginCursorOver`
  (params (TouchedComponent :type "PrimitiveComponent Object Reference"))
  (bind _returnvalue (`self.K2_GetActorLocation`))
  (set `self.Startlocation` _returnvalue)
  (set `self.TargetLocation_Up` (+ _returnvalue (0.0 0.0 20.0)))
  (bind (_direction _floatoutput) (`Timeline|MoveTileUponHover`)
    (:`Update`
      (`self.K2_SetActorLocation` (`KismetMathLibrary.VLerp` (`self.Startlocation`) (`self.TargetLocation_Up`) _floatoutput)))))

(event `OnEndCursorOver_Event`
  (params (TouchedActor :type "Actor Object Reference"))
  (`Timeline|MoveTileDown`
    (:`Update`
      (`self.K2_SetActorLocation` (`KismetMathLibrary.VLerp` (`self.TargetLocation_Up`) (`self.Startlocation`))))))

(fn `UserConstructionScript`)