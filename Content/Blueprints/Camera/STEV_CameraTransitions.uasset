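; State Tree evaluator that switches the camera between its in-round and in-shop states based on the game's state.
; Each tick it reads the GameState tag container from BP_GameInstance and requests the in-round state if it has GameState.Inround or a child tag, otherwise the in-shop state.
; It then prints the tag container every tick as debug output.
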(event `self.ReceiveTick`
  (params (DeltaTime :type "Float (single-precision)"))
  (`|ExecutionSequence`
    (:`then_0`
      (bind _asbp_game_instance (cast `/Game/Blueprints/Core/BP_GameInstance` (`GameplayStatics.GetGameInstance`)))
      (set `self.Game State` (`/Game/Blueprints/Core/BP_GameInstance.GameState` _asbp_game_instance))
      (if (`BlueprintGameplayTagLibrary.HasTag` (`self.Game State`) (struct :`TagName` "GameState.Inround"))
        (`self.RequestTransition` (`self.InroundState`))
        (else
          (`self.RequestTransition` (`self.InshopState`)))))
    (:`then_1`
      (`KismetSystemLibrary.PrintString` (`BlueprintGameplayTagLibrary.GetDebugStringFromGameplayTagContainer` (`self.Game State`))))))