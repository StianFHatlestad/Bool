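; BP_Goldball is the gold color ball Blueprint, which defines the effect played when the ball is pocketed.
; PlayPocketEffect spawns the NS_BallPotBasic Niagara system at the ball's location.
; It feeds the system the pocketed hole's XY at a fixed height, the normalized 2D ball velocity and the ball material.
; The construction script only calls the parent, and the other event stubs are disabled.
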(event `self.PlayPocketEffect`
  (params (PocketID :type Integer) (PocketActor :type "/Game/Blueprints/Core/BP_Pocket Object Reference"))
  (bind _returnvalue (`NiagaraFunctionLibrary.SpawnSystemAtLocation` "/Game/VFX/Niagara/Systems/PottingEffects/NS_BallPotBasic.NS_BallPotBasic" (`self.K2_GetActorLocation`)))
  (`|ExecutionSequence`
    (:`then_0`
      (`NiagaraComponent.SetVariablePosition` _returnvalue "Pocket" (`KismetMathLibrary.MakeVector` (.x (`self.K2_GetActorLocation` (`self.PocketedHole`))) (.y (`self.K2_GetActorLocation` (`self.PocketedHole`))) -20.0)))
    (:`then_1`
      (`NiagaraComponent.SetVariableVec3` _returnvalue "VelForward" (`KismetMathLibrary.Vector_Normal2D` (`self.GetBallVelocity`))))
    (:`then_2`
      (`NiagaraComponent.SetVariableMaterial` _returnvalue "Ballmat" (`self.BallMat`)))))

(fn `UserConstructionScript`
  (`parent.UserConstructionScript`))