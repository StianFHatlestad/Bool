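; BP_GreenBall is a colored ball that carries merge and split logic for its Multiplier and merged-ball index list, plus a Niagara pocket effect.
; Combine makes the faster ball destroy the slower after writing the multiplied value onto that doomed ball.
; TrySplit spawns a sibling, dividing the Multiplier by index-count parity and moving some indexes across.
; Both collision events are empty, their merge and split triggers disconnected, as is the index-append step.
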(event `self.ReceiveBeginPlay`
  (`parent.ReceiveBeginPlay`)
  (`|ExecutionSequence`))

(event `self.ReceiveActorBeginOverlap`
  (params (OtherActor :type "Actor Object Reference"))
  (`parent.ReceiveActorBeginOverlap` OtherActor))

(event `Combine`
  (params (`Last Collided Ball` :type "/Game/Blueprints/Balls/BP_Ball Object Reference"))
  (bind _lastcollidedgreenball (`self.lastCollidedGreenball`))
  ;[1 1 1] Combine Balls and adjust values
  (bind _asbp_green_ball (cast `/Game/Blueprints/Balls/ColorBalls/Green/BP_GreenBall` `Last Collided Ball`))
  (bind _output_get (set `self.lastCollidedGreenball` _asbp_green_ball))
  (if (> (`KismetMathLibrary.VSize` (`self.GetBallVelocity`)) (`KismetMathLibrary.VSize` (`self.GetBallVelocity` (`self.lastCollidedGreenball`))))
    (bind (_name _score _multiplier _weight _money _category _ballclass _price _statetags _interactiontags _uppgradetags _material) (break `/Game/Blueprints/Balls/S_GameplayAttributes` (`/Game/Blueprints/Balls/BP_Ball.S_GameplayAttributes` _output_get)))
    (set `/Game/Blueprints/Balls/BP_Ball.S_GameplayAttributes` (make `/Game/Blueprints/Balls/S_GameplayAttributes` _name _score (* _multiplier (`.Multiplier_17_3C2B5DEB43E99E7B3409C5BD59B45F38` (break `/Game/Blueprints/Balls/S_GameplayAttributes` (`self.S_GameplayAttributes`)))) _weight _money _category _ballclass _price (struct) _interactiontags _uppgradetags _material) _lastcollidedgreenball)
    (`self.K2_DestroyActor` _lastcollidedgreenball)
    (`KismetSystemLibrary.PrintString` (`KismetStringLibrary.Conv_IntToString` (`KismetArrayLibrary.Array_Length` (`self.MergedBallIndexes`))) true true (struct :`R` 1.0 :`B` 0.125984 :`A` 1.0) 2.0 "SPLITS")))

(event `Try Split`
  (params (`Spawn Transform Location` :type "Vector Structure"))
  ;[1 1 1] Run Split logic
  (if (> (`KismetArrayLibrary.Array_Length` (`self.MergedBallIndexes`)) 2)
    (bind _returnvalue (`|SpawnActorFromClass` "BP_GreenBall_C" (`KismetMathLibrary.MakeTransform` `Spawn Transform Location` (struct :`Roll` -90.0)) "Undefined" "MultiplyWithRoot" null null))
    (set `self.LastSplitSibling` _returnvalue)
    (`|ExecutionSequence`
      (:`then_0`
        (`|ExecutionSequence`
          (:`then_0`
            (if (> (`KismetArrayLibrary.Array_Length` (`self.MergedBallIndexes`)) 1)
              (if (== (mod (`KismetArrayLibrary.Array_Length` (`self.MergedBallIndexes`)) 2) 1)
                (`self.Fraction (THIRD)`)
                (`self.Split Merged Ball Indexes`)
                (else
                  (`self.Halve`)
                  (`self.Split Merged Ball Indexes`)))
              (else
                (`self.Halve`)))))))))

(event `Halve`
  (bind (_s_gameplayattributes_name _s_gameplayattributes_score _s_gameplayattributes_multiplier _s_gameplayattributes_weight _s_gameplayattributes_money _s_gameplayattributes_category _s_gameplayattributes_ballclass _s_gameplayattributes_price _s_gameplayattributes_statetags _s_gameplayattributes_interactiontags _s_gameplayattributes_uppgradetags _s_gameplayattributes_material) (break `/Game/Blueprints/Balls/S_GameplayAttributes` (`self.S_GameplayAttributes`)))
  ;[1 1 1] Result: EVEN OR 0
  (bind _output_get (set `/Game/Blueprints/Balls/BP_Ball.S_GameplayAttributes` (make `/Game/Blueprints/Balls/S_GameplayAttributes` _s_gameplayattributes_name _s_gameplayattributes_score (/ _s_gameplayattributes_multiplier 2.0) _s_gameplayattributes_weight _s_gameplayattributes_money _s_gameplayattributes_category _s_gameplayattributes_ballclass _s_gameplayattributes_price (struct) _s_gameplayattributes_interactiontags _s_gameplayattributes_uppgradetags _s_gameplayattributes_material) (`self.LastSplitSibling`)))
  (set `self.S_GameplayAttributes` _output_get))

(event `Fraction (Third)`
  (bind (_s_gameplayattributes_name _s_gameplayattributes_score _s_gameplayattributes_multiplier _s_gameplayattributes_weight _s_gameplayattributes_money _s_gameplayattributes_category _s_gameplayattributes_ballclass _s_gameplayattributes_price _s_gameplayattributes_statetags _s_gameplayattributes_interactiontags _s_gameplayattributes_uppgradetags _s_gameplayattributes_material) (break `/Game/Blueprints/Balls/S_GameplayAttributes` (`self.S_GameplayAttributes`)))
  (bind _returnvalue (/ _s_gameplayattributes_multiplier 3.0))
  ;[1 1 1] Result: UN-EVEN
  (bind _output_get (set `/Game/Blueprints/Balls/BP_Ball.S_GameplayAttributes` (make `/Game/Blueprints/Balls/S_GameplayAttributes` _s_gameplayattributes_name _s_gameplayattributes_score _returnvalue _s_gameplayattributes_weight _s_gameplayattributes_money _s_gameplayattributes_category _s_gameplayattributes_ballclass _s_gameplayattributes_price (struct) _s_gameplayattributes_interactiontags _s_gameplayattributes_uppgradetags _s_gameplayattributes_material) (`self.LastSplitSibling`)))
  (set `self.S_GameplayAttributes` (make `/Game/Blueprints/Balls/S_GameplayAttributes` (break `/Game/Blueprints/Balls/S_GameplayAttributes` _output_get) (`.Score_2_2598F13C43221B678AD096920341C0C7` (break `/Game/Blueprints/Balls/S_GameplayAttributes` _output_get)) (* _returnvalue 2.0) (`.Weight_5_3D57DC754599AEAC0FD22E837ADB94E9` (break `/Game/Blueprints/Balls/S_GameplayAttributes` _output_get)) (`.Money_44_A5F9D60845ED44E0E02D31B4A1DECEE0` (break `/Game/Blueprints/Balls/S_GameplayAttributes` _output_get)) (`.Category_14_16EB49B74E54F76EB6ED01A647D64054` (break `/Game/Blueprints/Balls/S_GameplayAttributes` _output_get)) (`.BallClass_22_BF39C1D54109D681211D04AC27E726D3` (break `/Game/Blueprints/Balls/S_GameplayAttributes` _output_get)) (`.Price_25_16B268964FF0D80118E4279EB5B5841A` (break `/Game/Blueprints/Balls/S_GameplayAttributes` _output_get)) (struct) (`.InteractionTags_34_1D59837F44DE8A509B65CAABE75AD771` (break `/Game/Blueprints/Balls/S_GameplayAttributes` _output_get)) (`.UppgradeTags_37_44DF3FA74EADD10B244A43AE60259F52` (break `/Game/Blueprints/Balls/S_GameplayAttributes` _output_get)) (`.Material_40_56E5DA014ACBE816108ECB86250EE554` (break `/Game/Blueprints/Balls/S_GameplayAttributes` _output_get)))))

(event `Split Merged Ball Indexes`
  (bind _lastsplitsibling (`self.LastSplitSibling`))
  (bind _mergedballindexes (`self.MergedBallIndexes`))
  (bind _returnvalue (`KismetArrayLibrary.Array_Length` (`self.MergedBallIndexes`)))
  (bind _returnvalue_2 (+ (/ _returnvalue 2) (mod _returnvalue 2)))
  ;[1 1 1] Split Array
  (for (_array_element _array_index) (`self.MergedBallIndexes`)
    (if (>= _returnvalue_2 _array_index)
      (if (== _array_index (+ _returnvalue_2 1))
        (set `/Game/Blueprints/Balls/BP_Ball.BallNumber` _array_element _lastsplitsibling)
        (`KismetArrayLibrary.Array_Remove` (`self.MergedBallIndexes`) _array_index)
        (`self.Set First Merged Ball Index` _lastsplitsibling)
        (`KismetSystemLibrary.PrintString` (`KismetStringLibrary.Conv_IntToString` (`KismetArrayLibrary.Array_Length` (`self.MergedBallIndexes`))) true true (struct :`R` 1.0 :`B` 0.125984 :`A` 1.0) 2.0 "SPLITS")
        (`self.SetParams` (`self.LastSplitSibling`))
        (else
          (`|ExecutionSequence`
            (:`then_0`
              (`KismetArrayLibrary.Array_Add` (`/Game/Blueprints/Balls/ColorBalls/Green/BP_GreenBall.MergedBallIndexes` (`self.LastSplitSibling`)) (`|GetArrayItem` _mergedballindexes _array_element))
              (`KismetArrayLibrary.Array_Remove` _mergedballindexes _array_index))))))))

(event `Set First Merged Ball Index`
  ;[1 1 1] Set first index on merged balls
)

(event `self.BallCollision`
  ;[1 1 1] Start Merge
)

(event `self.AnyCollision`
  (params (`Collision Interaction Tags` :type "GameplayTagContainer Structure") (`First Or Final Execution` :type Boolean))
  ;[1 1 1] Start Split
)

(event `self.PlayPocketEffect`
  (params (PocketID :type Integer) (PocketActor :type "/Game/Blueprints/Core/BP_Pocket Object Reference"))
  (bind _returnvalue (`NiagaraFunctionLibrary.SpawnSystemAtLocation` "/Game/VFX/Niagara/Systems/PottingEffects/NS_BallPotBasic.NS_BallPotBasic" (`self.K2_GetActorLocation`)))
  (`|ExecutionSequence`
    (:`then_0`
      (`NiagaraComponent.SetVariablePosition` _returnvalue "Pocket" (`KismetMathLibrary.MakeVector` (.x (`self.K2_GetActorLocation` (`self.PocketedHole`))) (.y (`self.K2_GetActorLocation` (`self.PocketedHole`))) -20.0)))
    (:`then_1`
      (`NiagaraComponent.SetVariableVec3` _returnvalue "VelForward" (`KismetMathLibrary.Vector_Normal2D` (`self.GetBallVelocity`))))
    (:`then_2`
      (`NiagaraComponent.SetVariableMaterial` _returnvalue "Ballmat" (`self.BallMat`)))))

(fn `UserConstructionScript`
  (`parent.UserConstructionScript`))