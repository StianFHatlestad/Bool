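; BP_RedBall is an explosive colour ball that counts down a fuse on each Trigger and blasts on collision once primed.
; Tick adds a Primed gameplay tag when the fuse runs out, and AnyCollision checks that tag before calling Blast.
; Blast spawns a Niagara effect, sphere-traces for BP_Balls to push outward with scaled velocity, randomly kicks itself, then resets the fuse and tag.
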(event `self.ReceiveBeginPlay`
  (`parent.ReceiveBeginPlay`)
  (`self.ResetFuse`))

(event `Blast`
  (bind _returnvalue (`self.K2_GetActorLocation`))
  (bind _returnvalue_2 (`self.K2_GetActorLocation`))
  ;[1 1 1] Blast
  (`|ExecutionSequence`
    (:`then_0`
      (`NiagaraFunctionLibrary.SpawnSystemAtLocation` "/Game/VFX/Niagara/Systems/NS_Blast.NS_Blast" (`self.K2_GetActorLocation`) (struct) (0.5 0.5 0.5)))
    (:`then_1`
      (bind _outhits (`KismetSystemLibrary.SphereTraceMulti` _returnvalue_2 _returnvalue_2 (`self.BlastRadius`) "TraceTypeQuery1"))
      (for _array_element _outhits
        (bind (_bblockinghit _binitialoverlap _time _distance _location _impactpoint _normal _impactnormal _physmat _hitactor) (`GameplayStatics.BreakHitResult` _array_element))
        (bind _asbp_ball (cast `/Game/Blueprints/Balls/BP_Ball` _hitactor))
        (bind _returnvalue_3 (`self.K2_GetActorLocation` _hitactor))
        (`self.SetBallVelocity` _asbp_ball (+ (`self.GetBallVelocity` _asbp_ball) (* (* (`KismetMathLibrary.GetForwardVector` (`KismetMathLibrary.FindLookAtRotation` _returnvalue _returnvalue_3)) (`self.BlastStrength`)) (`KismetMathLibrary.MapRangeClamped` (* (/ (`KismetMathLibrary.VSize` (- (`KismetMathLibrary.Normal` _returnvalue) (`KismetMathLibrary.Normal` _returnvalue_3))) (`self.BlastRadius`)) 100.0) 0.0 1.0 1.0))))
        (`self.SetBallVelocity` (+ (`self.GetBallVelocity`) (* (`KismetMathLibrary.MakeVector` (`KismetMathLibrary.RandomFloatInRange` -1.0 1.0) (`KismetMathLibrary.RandomFloatInRange` -1.0 1.0)) (`self.BlastStrength`))))))
    (:`then_3`
      (`self.ResetFuse`))))

(event `ResetFuse`
  (bind (_s_ball_name _s_ball_score _s_ball_multiplier _s_ball_weight _s_ball_money _s_ball_category) (break `/Game/Blueprints/Balls/S_Ball` (`self.S_ball`)))
  ;[1 1 1] Restart
  (`|ExecutionSequence`
    (:`then_0`
      (set `self.Fuse` (`self.FuseMax`)))
    (:`then_1`
      (`BlueprintGameplayTagLibrary.RemoveGameplayTag` _s_ball_category (struct :`TagName` "Ball.ObjectBall.Color.Red.Primed")))))

(event `self.ReceiveTick`
  (params (DeltaSeconds :type "Float (single-precision)"))
  (bind (_s_ball_name _s_ball_score _s_ball_multiplier _s_ball_weight _s_ball_money _s_ball_category) (break `/Game/Blueprints/Balls/S_Ball` (`self.S_ball`)))
  ;[1 1 1] Prepare to explode
  (if (<= (`self.Fuse`) 0)
    (`BlueprintGameplayTagLibrary.AddGameplayTag` _s_ball_category (struct :`TagName` "Ball.ObjectBall.Color.Red.Primed"))))

(event `self.Trigger`
  (bind _fuse (`self.Fuse`))
  ;[1 1 1] Triggering Collision
  (`/Engine/EditorBlueprintResources/StandardMacros.DecrementInt` _fuse
    (:`  `
      (`KismetSystemLibrary.PrintString` (`KismetStringLibrary.Conv_IntToString` _fuse) true true (struct :`R` 1.0 :`B` 0.048309 :`A` 1.0)))))

(event `self.BallCollider`
  ;[1 1 1] Trigger Blast
)

(event `self.AnyCollision`
  (bind (_s_ball_name _s_ball_score _s_ball_multiplier _s_ball_weight _s_ball_money _s_ball_category) (break `/Game/Blueprints/Balls/S_Ball` (`self.S_ball`)))
  ;[1 1 1] Trigger Blast
  (if (`BlueprintGameplayTagLibrary.HasTag` _s_ball_category (struct :`TagName` "Ball.ObjectBall.Color.Red.Primed"))
    (`self.Blast`)))

(fn `UserConstructionScript`
  (`parent.UserConstructionScript`))