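; Short-lived component in the red color ball folder that paints a fading, shrinking smoke trail into the RT_Cloud render target at its owner's location.
; Each tick it lowers density and radius at constant rates, then draws PaintMat onto the canvas.
; Paint scales position and radius by the target mesh's vertical extent and supports an erase mode.
; The component destroys itself one second after BeginPlay.
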(event `self.ReceiveBeginPlay`
  (`KismetSystemLibrary.Delay` 1.0)
  (`self.K2_DestroyComponent`))

(event `self.ReceiveTick`
  (params (DeltaSeconds :type "Float (single-precision)"))
  (`|ExecutionSequence`
    (:`then_0`
      (set `self.Density` (`KismetMathLibrary.FInterpTo_Constant` (`self.Density`) 0.0 DeltaSeconds (`self.FadeRate`))))
    (:`then_1`
      (set `self.Radius` (`KismetMathLibrary.FInterpTo_Constant` (`self.Radius`) 0.0 DeltaSeconds (`self.ShrinkRate`))))
    (:`then_2`
      (`self.Paint` "/Game/VFX/RaymarchedSmokes/TestRenderTargets/RT_Cloud.RT_Cloud" (`Actor.K2_GetActorLocation` (`self.GetOwner`)) false (`self.Density`) (`self.Radius`) (`self.Target Mesh`)))))

(fn `Paint`
  (params (TextureRenderTarget :type "TextureRenderTarget2D Object Reference") (Position :type "Vector Structure") (Erase :type Boolean) (Density :type "Float (double-precision)") (Radius :type "Float (double-precision)") (TargetMesh :type "Actor Object Reference"))
  (locals (Size :type "Vector2D Structure") (Context :type "DrawToRenderTargetContext Structure") (Canvas :type "Canvas Object Reference"))
  (bind (_canvas _size _context) (`KismetRenderingLibrary.BeginDrawCanvasToRenderTarget` TextureRenderTarget))
  (set `self.Size_0` _size)
  (set `self.Context_0` _context)
  (set `self.Canvas_0` _canvas)
  (`MaterialInstanceDynamic.SetVectorParameterValue` (`self.PaintMat`) "PaintCenter" (`KismetMathLibrary.Conv_VectorToLinearColor` (/ (`local.Position`) (.z (`.BoxExtent` (`Actor.GetActorBounds` (`local.TargetMesh`) false false))))))
  (`MaterialInstanceDynamic.SetScalarParameterValue` (`self.PaintMat`) "Density" (`KismetMathLibrary.SelectFloat` -1000.0 (`local.Density`) (`local.Erase`)))
  (`MaterialInstanceDynamic.SetScalarParameterValue` (`self.PaintMat`) "Radius" (/ (`local.Radius`) (.z (`.BoxExtent` (`Actor.GetActorBounds` (`local.TargetMesh`) false false)))))
  (`Canvas.K2_DrawMaterial` (`self.Canvas_0`) (`self.PaintMat`) (0.0 0.0) (`self.Size_0`) (0.0 0.0) (1.0 1.0) 0.0 (0.5 0.5))
  (`KismetRenderingLibrary.EndDrawCanvasToRenderTarget` (`self.Context_0`)))