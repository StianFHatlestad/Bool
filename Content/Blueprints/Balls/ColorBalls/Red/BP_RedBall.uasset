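; Red object ball that turns into a bomb after being triggered enough times.
; Each trigger burns its fuse until a delayed prime sets a gameplay tag, smoke and material glow.
; Its first collision while primed sphere-traces and shoves nearby balls, boosts itself, paints smoke into a render target and resets the fuse.
; The Defuser upgrade tag makes priming raise the multiplier and resetting lower it.
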(event `self.ReceiveTick`
  (params (DeltaSeconds :type "Float (single-precision)"))
  ;[1 1 1] Tick
  (`|ExecutionSequence`))

(event `self.ReceiveBeginPlay`
  (`parent.ReceiveBeginPlay`)
  (`|ExecutionSequence`
    (:`then_1`
      (`self.ResetFuse`))))

(event `self.PlayPocketEffect`
  (params (PocketID :type Integer) (PocketActor :type "/Game/Blueprints/Core/BP_Pocket Object Reference"))
  ; PocketingVisuals
  (bind _returnvalue (`NiagaraFunctionLibrary.SpawnSystemAtLocation` "/Game/VFX/Niagara/Systems/PottingEffects/NS_BallPotBasic.NS_BallPotBasic" (`self.K2_GetActorLocation`)))
  (`|ExecutionSequence`
    (:`then_0`
      (`NiagaraComponent.SetVariablePosition` _returnvalue "Pocket" (`KismetMathLibrary.MakeVector` (.x (`self.K2_GetActorLocation` (`self.PocketedHole`))) (.y (`self.K2_GetActorLocation` (`self.PocketedHole`))) -20.0)))
    (:`then_1`
      (`NiagaraComponent.SetVariableVec3` _returnvalue "VelForward" (`KismetMathLibrary.Vector_Normal2D` (`self.GetBallVelocity`))))
    (:`then_2`
      (`NiagaraComponent.SetVariableMaterial` _returnvalue "Ballmat" (`self.BallMat`)))))

(event `Defuser`
  ;[1 1 1 0.5] Defuser Logic
  ;; Has Defuser Upgrade?
  (if (`BlueprintGameplayTagLibrary.HasTag` (`.UppgradeTags_37_44DF3FA74EADD10B244A43AE60259F52` (break `/Game/Blueprints/Balls/S_GameplayAttributes` (`self.S_GameplayAttributes`))) (struct :`TagName` "Ball.ObjectBall.Color.Red.Upgrades.Defuser"))
    ;; CheckIfPrimedOrUnprimed
    (if (`BlueprintGameplayTagLibrary.HasTag` (`.StateTags_47_C7AFFCA64CA55D5277DC4999C49523CB` (break `/Game/Blueprints/Balls/S_GameplayAttributes` (`self.S_GameplayAttributes`))) (struct :`TagName` "Ball.ObjectBall.Color.Red.Primed"))
      ;; Add 1 To multiplier
      (setmembers `/Game/Blueprints/Balls/S_GameplayAttributes` :`StructRef` (`self.S_GameplayAttributes`) :`Multiplier` (+ (`.Multiplier_17_3C2B5DEB43E99E7B3409C5BD59B45F38` (break `/Game/Blueprints/Balls/S_GameplayAttributes` (`self.S_GameplayAttributes`))) 1.0))
      (else
        ;; Subtract 1 from multiplier
        (setmembers `/Game/Blueprints/Balls/S_GameplayAttributes` :`StructRef` (`self.S_GameplayAttributes`) :`Multiplier` (- (`.Multiplier_17_3C2B5DEB43E99E7B3409C5BD59B45F38` (break `/Game/Blueprints/Balls/S_GameplayAttributes` (`self.S_GameplayAttributes`))) 1.0))))))

(event `prime`
  ;[1 1 1] Prepare To blast
  (`KismetSystemLibrary.Delay` (`self.PrimingTime`))
  ;; Adds the prime tag
  (`BlueprintGameplayTagLibrary.AddGameplayTag` (`.StateTags_47_C7AFFCA64CA55D5277DC4999C49523CB` (break `/Game/Blueprints/Balls/S_GameplayAttributes` (`self.S_GameplayAttributes`))) (struct :`TagName` "Ball.ObjectBall.Color.Red.Primed"))
  (`|ExecutionSequence`
    (:`then_0`
      ;; Event For Defuser Upgrade
      (`self.Defuser`))
    (:`then_1`
      ;; Visual effect for priming
      (`MaterialInstanceDynamic.SetScalarParameterValue` (`self.BallMat`) "Primed" 1.0)
      (`NiagaraComponent.SetVariableFloat` (`self.PrimedSmoke`) "SpawnRate" 8.0))))

(event `ResetFuse`
  ;[1 1 1] Reset Fuse
  ;; Comment
  (set `self.Fuse` (`self.FuseMax`))
  (`BlueprintGameplayTagLibrary.RemoveGameplayTag` (`.StateTags_47_C7AFFCA64CA55D5277DC4999C49523CB` (break `/Game/Blueprints/Balls/S_GameplayAttributes` (`self.S_GameplayAttributes`))) (struct :`TagName` "Ball.ObjectBall.Color.Red.Primed"))
  (`|ExecutionSequence`
    (:`then_0`
      ;; Event For Defuser Upgrade
      (`self.Defuser`))
    (:`then_1`
      ;; Visual Reset From Prime
      (`NiagaraComponent.SetVariableFloat` (`self.PrimedSmoke`) "SpawnRate" 0.0))
    (:`then_2`
      (bind _ballmat (`self.BallMat`)
        (:`then`
          (`MaterialInstanceDynamic.SetScalarParameterValue` _ballmat "Primed" 0.0))
        (:`else`)))))

(event `Blast`
  (bind _returnvalue (`self.GetBallVelocity`))
  ;[1 1 1] Blast
  (if (`BlueprintGameplayTagLibrary.HasTag` (`.StateTags_47_C7AFFCA64CA55D5277DC4999C49523CB` (break `/Game/Blueprints/Balls/S_GameplayAttributes` (`self.S_GameplayAttributes`))) (struct :`TagName` "Ball.ObjectBall.Color.Red.Primed"))
    (`|ExecutionSequence`
      (:`then_0`
        ;; DisplaceOthers then DisplaceSelf
        (`self.Blast TraceTargets`))
      (:`then_1`
        (`self.SetBallVelocity` (+ _returnvalue (* (`self.BlastStrength`) (`KismetMathLibrary.Normal` _returnvalue)))))
      (:`then_2`
        ;; Visuals
        (`NiagaraFunctionLibrary.SpawnSystemAtLocation` "/Game/VFX/Niagara/Systems/Explosions/Blast/NS_Blastv2.NS_Blastv2" (`self.K2_GetActorLocation`) (struct) (0.5 0.5 0.5))
        (`GameplayStatics.PlayWorldCameraShake` "/Game/VFX/CameraShake/CS_RedballBlastShake.CS_RedballBlastShake_C" (`self.K2_GetActorLocation`) 0.0 20000.0 1.0 true))
      (:`then_3`
        (bind (_direction _pufftrack) (`Timeline|Timeline` :!via `PlayFromStart`)
          (:`Update`
            (`self.Paint` "/Game/VFX/RaymarchedSmokes/TestRenderTargets/RT_Cloud.RT_Cloud" (`self.K2_GetActorLocation`) false (* (`self.PuffDensity`) _pufftrack) (* (`self.PuffRadius`) _pufftrack) (`self.TargetMesh`)))))
      (:`then_4`
        ;; Reset Fuse
        (`self.ResetFuse`))
      (:`then_5`
        (`GameplayStatics.PlaySoundAtLocation` "/Game/SFX/Balls/Bomb/BombBlast_Wav_Cue.BombBlast_Wav_Cue" (`self.K2_GetActorLocation`) (struct) 1.0 1.0 0.0 null null null null)))))

(event `Blast TraceTargets`
  (bind _returnvalue (`self.K2_GetActorLocation`))
  (bind _returnvalue_2 (`self.K2_GetActorLocation`))
  (bind _returnvalue_3 (`self.K2_GetActorLocation` (`self.BlastedBall`)))
  (bind _returnvalue_4 (* (/ (`KismetMathLibrary.Abs` (`KismetMathLibrary.VSize` (`KismetMathLibrary.Normal` (- _returnvalue _returnvalue_3)))) (`self.BlastRadius`)) (`self.BlastStrength`)))
  ;[1 1 1] Blast
  ;; Find Affected Balls
  (bind _outhits (`KismetSystemLibrary.SphereTraceMulti` _returnvalue_2 _returnvalue_2 (`self.BlastRadius`) "TraceTypeQuery1"))
  (for _array_element _outhits
    (bind _asbp_ball (cast `/Game/Blueprints/Balls/BP_Ball` (`.HitActor` (`GameplayStatics.BreakHitResult` _array_element))))
    (set `self.BlastedBall` _asbp_ball)
    (`self.BlastedBall`
      (:`then`
        (`|ExecutionSequence`
          (:`then_0`
            ;; This Is what offsets Other balls
            (`self.SetBallVelocity` (`self.BlastedBall`) (+ (`self.GetBallVelocity` (`self.BlastedBall`)) (* (* (`KismetMathLibrary.GetForwardVector` (`KismetMathLibrary.FindLookAtRotation` _returnvalue _returnvalue_3)) _returnvalue_4) _returnvalue_4))))
          (:`then_1`
            ;; Volumetric Smoke Trail
            (`|ExecutionSequence`
              (:`then_0`
                (bind _returnvalue_5 (`AddComponent|NODE_AddBP_SmokingComponent-1` :`self` (`self.BlastedBall`)))
                (set `self.CurrentModifiedPaintComp` _returnvalue_5))
              (:`then_1`
                (set `/Game/Blueprints/Balls/ColorBalls/Red/BP_SmokingComponent.PaintMat` (`/Game/Blueprints/Balls/BP_Ball.PaintMat` (`self.BlastedBall`)) (`self.CurrentModifiedPaintComp`)))
              (:`then_2`
                (set `/Game/Blueprints/Balls/ColorBalls/Red/BP_SmokingComponent.Density` 20.0 (`self.CurrentModifiedPaintComp`)))
              (:`then_3`
                (set `/Game/Blueprints/Balls/ColorBalls/Red/BP_SmokingComponent.Radius` 10.0 (`self.CurrentModifiedPaintComp`)))
              (:`then_4`
                (set `/Game/Blueprints/Balls/ColorBalls/Red/BP_SmokingComponent.Target Mesh` (`self.TargetMesh`) (`self.CurrentModifiedPaintComp`)))))))
      (:`else`))))

(fn `First AnyCollision`
  (params (`Interaction Payload` :type "GameplayTagContainer Structure"))
  (`parent.First AnyCollision` `Interaction Payload`)
  ; If Primed trigger blast
  (`self.Blast`))

(fn `Triggered`
  (`parent.Triggered`)
  ; Check If Priming
  (if (not (`BlueprintGameplayTagLibrary.HasTag` (`.StateTags_47_C7AFFCA64CA55D5277DC4999C49523CB` (break `/Game/Blueprints/Balls/S_GameplayAttributes` (`self.S_GameplayAttributes`))) (struct :`TagName` "Ball.ObjectBall.Color.Red.Primed")))
    ; Decrement Fuse
    (set `self.Fuse` (- (`self.Fuse`) 1))
    ; Check if fuse is 0
    (if (== (`self.Fuse`) 0)
      (`self.prime`))))

(fn `UserConstructionScript`
  (`parent.UserConstructionScript`))