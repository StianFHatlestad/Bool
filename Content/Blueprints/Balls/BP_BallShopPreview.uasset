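; BP_BallShopPreview is a preview ball actor, apparently for the shop, that shows a given ball number and color on a skeletal mesh.
; On BeginPlay it creates a dynamic instance of MM_Ballmat on the mesh and stores it as BallMat.
; BallNumber and BallColor then drive that material's Number and Basetype scalar parameters, with no further runtime logic.
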(event `self.ReceiveBeginPlay`
  (bind _returnvalue (`PrimitiveComponent.CreateDynamicMaterialInstance` (`self.SkeletalMesh`) 0 "/Game/Materials/Balls/MM_Ballmat.MM_Ballmat" "None"))
  (set `self.BallMat` _returnvalue)
  (`|ExecutionSequence`
    (:`then_0`
      (`MaterialInstanceDynamic.SetScalarParameterValue` (`self.BallMat`) "Number" (`KismetMathLibrary.Conv_IntToDouble` (`self.BallNumber`))))
    (:`then_1`
      (`MaterialInstanceDynamic.SetScalarParameterValue` (`self.BallMat`) "Basetype" (`KismetMathLibrary.Conv_IntToDouble` (`self.BallColor`))))))

(fn `UserConstructionScript`)