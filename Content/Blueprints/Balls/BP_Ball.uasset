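; Base ball actor for a pool-style game, with material and trail visuals set from its gameplay attributes.
; Hits fetch the other actor's attributes through BP_BallInteract, and CollisionHandler walks ball and obstacle tag hierarchies into layered response events with mostly empty General hooks.
; Interaction tags also feed TryInteract, which calls an empty Triggered hook.
; Pocketed balls either reset or teleport below the table; a Paint helper draws into render targets.
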(event `self.ReceiveBeginPlay`
  (`parent.ReceiveBeginPlay`)
  (`|ExecutionSequence`
    (:`then_0`
      (bind _returnvalue (`KismetMaterialLibrary.CreateDynamicMaterialInstance` "/Game/VFX/RaymarchedSmokes/M_VolumePaint.M_VolumePaint"))
      (set `self.PaintMat` _returnvalue))
    (:`then_1`
      (bind _outactors (`GameplayStatics.GetAllActorsWithTag` "VolumeTarget"))
      (for _array_element _outactors
        (set `self.TargetMesh` _array_element)))))

(event `self.ReceiveTick`
  (params (DeltaSeconds :type "Float (single-precision)"))
  (`parent.ReceiveTick` DeltaSeconds)
  (`|ExecutionSequence`
    (:`then_0`
      (`self.Speedometer`))
    (:`then_1`
      (`self.DisableBallsBelowZ`))))

(event `Speedometer`
  ;[1 1 1 0.5] Set single float value for ball velocity
  (set `self.BallVelocityLength` (`KismetMathLibrary.VSize` (`self.GetBallVelocity`))))

(event `SetParams`
  (bind (_name _score _multiplier _weight _money _category) (break `/Game/Blueprints/Balls/S_GameplayAttributes` (`self.S_GameplayAttributes`)))
  (`|ExecutionSequence`
    (:`then_0`
      ;[1 1 1] Visual
      (if (`BlueprintGameplayTagLibrary.HasTag` _category (struct :`TagName` "Ball.ObjectBall.Color"))
        (for _array_element (`BlueprintGameplayTagLibrary.BreakGameplayTagContainer` _category)
          (`|SwitchGameplayTag` _array_element
            (:`Ball.ObjectBall.Color.Red`
              (`self.SetVisuals` 3))
            (:`Ball.ObjectBall.Color.Blue`
              (`self.SetVisuals` 4))
            (:`Ball.ObjectBall.Color.Yellow`
              (`self.SetVisuals` 5))
            (:`Ball.ObjectBall.Color.Green`
              (`self.SetVisuals` 7))))
        (else
          (`self.SetVisuals` (`self.BallColor`)))))
    (:`then_1`
      (set `self.InitialLocation` (`self.K2_GetActorLocation`)))))

(event `SetVisuals`
  (params (BallColor :type Integer))
  ;[1 1 1] Visual
  (`|ExecutionSequence`
    (:`then_0`
      (set `self.BallColor` BallColor))
    (:`then_1`
      (bind _returnvalue (`PrimitiveComponent.CreateDynamicMaterialInstance` (`self.MeshComponent`) 0 (`.Material_40_56E5DA014ACBE816108ECB86250EE554` (break `/Game/Blueprints/Balls/S_GameplayAttributes` (`self.S_GameplayAttributes`))) "None"))
      (set `self.BallMat` _returnvalue)
      (`|ExecutionSequence`
        (:`then_0`
          (`MaterialInstanceDynamic.SetScalarParameterValue` (`self.BallMat`) "Number" (`KismetMathLibrary.Conv_IntToDouble` (`self.BallNumber`))))
        (:`then_1`
          (`MaterialInstanceDynamic.SetScalarParameterValue` (`self.BallMat`) "Basetype" (`KismetMathLibrary.Conv_IntToDouble` (`self.BallColor`))))))
    (:`then_2`
      (`NiagaraComponent.SetVariableFloat` (`self.trail`) "Color" (`KismetMathLibrary.Conv_IntToDouble` (`self.BallColor`))))))

(event `SpawnImpact`
  (if (> (`KismetMathLibrary.VSize` (`self.GetBallVelocity`)) 50.0)
    (bind _returnvalue (`NiagaraFunctionLibrary.SpawnSystemAtLocation` "/Game/VFX/Niagara/Systems/NS_GeneralBallImpact.NS_GeneralBallImpact" (`.ImpactPoint` (`GameplayStatics.BreakHitResult` (`self.LastCollision`)))))
    (`NiagaraComponent.SetVariableFloat` _returnvalue "ImpactPower" (`KismetMathLibrary.MapRangeClamped` (`KismetMathLibrary.VSize` (`self.GetBallVelocity`)) 50.0 200.0 10.0 20.0))
    (`NiagaraComponent.SetVariableInt` _returnvalue "ImpactColor" (`self.BallColor`))))

(event `/Game/Blueprints/Balls/BP_BallInteract.RemoteInteraction`
  (params (InteractionPayload :type "GameplayTagContainer Structure"))
  ;[1 1 1 0.5] This happens when another actor forces an interaction without colliding (For example red ball explosion)
  (`self.TryInteract` InteractionPayload))

(event `TryInteract`
  (params (`Interaction Payload` :type "GameplayTagContainer Structure"))
  ;[1 1 1] Determine what kind of interaction is happening
  (for _array_element (`BlueprintGameplayTagLibrary.BreakGameplayTagContainer` `Interaction Payload`)
    (`|SwitchGameplayTag` _array_element
      (:`GameplayAttribute.Triggering`
        (`self.Triggered`)))))

(event `NonBallCollisionCommon`
  (`self.ObstacleCollision`)
  (`self.AudioEventWallCollision`))

(event `/Game/Blueprints/Balls/BP_BallInteract.Pocketed`
  (params (PocketID :type Integer) (PocketActor :type "/Game/Blueprints/Core/BP_Pocket Object Reference"))
  ; On Pocketed
  (set `self.PocketedHole` PocketActor)
  (`|ExecutionSequence`
    (:`then_0`
      (`self.PlayPocketEffect` PocketID PocketActor)
      (if (`BlueprintGameplayTagLibrary.HasTag` (`.InteractionTags_34_1D59837F44DE8A509B65CAABE75AD771` (break `/Game/Blueprints/Balls/S_GameplayAttributes` (`self.S_GameplayAttributes`))) (struct :`TagName` "GameplayAttribute.Respawning"))
        (`self.ResetPos`)
        (else
          (`self.SetActorActivatedState` false)
          (`self.PlayPocketEffect` 0 (`self.PocketedHole`)))))))

(event `AudioEventWallCollision`
  (`GameplayStatics.PlaySoundAtLocation` (`self.WallCollisionCue`) (`self.K2_GetActorLocation`) (struct) (`KismetMathLibrary.MapRangeClamped` (`KismetMathLibrary.VSize` (`self.GetBallVelocity`)) 0.0 200.0 0.0 1.0) 1.0 0.0 null null null null))

(event `AudioEventBallCollision`
  (`GameplayStatics.PlaySoundAtLocation` (`self.BallCollisionCue`) (`self.K2_GetActorLocation`) (struct) (`KismetMathLibrary.MapRangeClamped` (`KismetMathLibrary.VSize` (`self.GetBallVelocity`)) 0.0 200.0 0.0 1.0) 1.0 0.0 null null null null))

(event `PlayPocketEffect`
  (params (PocketID :type Integer) (PocketActor :type "/Game/Blueprints/Core/BP_Pocket Object Reference")))

(event `ResetPos`
  (`|ExecutionSequence`
    (:`then_0`
      (`self.SetBallVelocity` (0.0 0.0 0.0))
      (`self.SetBallAngularVelocity` (`KismetMathLibrary.MakeRotator` 0.0)))
    (:`then_1`
      (`self.K2_SetActorLocation` (`self.InitialLocation`) false true))))

(event `AnyCollision`
  (params (`Collision Interaction Tags` :type "GameplayTagContainer Structure") (`First Or Final Execution` :type Boolean))
  ;[1 1 1] All Possible Responses
  ;; General
  (if `First Or Final Execution`
    (`self.First AnyCollision` `Collision Interaction Tags`)))

(event `self.SphereComponent.OnComponentHit`
  (params (HitComponent :type "PrimitiveComponent Object Reference") (OtherActor :type "Actor Object Reference") (OtherComp :type "PrimitiveComponent Object Reference") (NormalImpulse :type "Vector Structure") (Hit :type "HitResult Structure (by ref)"))
  ;[1 1 1] Logic For Deciding Proper Collision Response
  ;; Check if collided object implements ballinteraction interface, if so, return gameplay attributes and trigger the general collision event
  (set `self.last Collided Actor` OtherActor)
  (set `self.LastCollision` Hit)
  (if (`KismetSystemLibrary.DoesImplementInterface` (`.HitActor` (`GameplayStatics.BreakHitResult` (`self.LastCollision`))) "/Game/Blueprints/Balls/BP_BallInteract.BP_BallInteract_C")
    (bind _gameplayattributes (message `/Game/Blueprints/Balls/BP_BallInteract.ReturnAllRelevantCollisionData` (`self.last Collided Actor`)))
    (set `self.LastCollidedAttributes` _gameplayattributes)
    (`|ExecutionSequence`
      (:`then_0`
        (`self.CollisionHandler` (`self.LastCollision`) (`self.LastCollidedAttributes`))
        (`self.AnyCollision` (`.InteractionTags_34_1D59837F44DE8A509B65CAABE75AD771` (break `/Game/Blueprints/Balls/S_GameplayAttributes` (`self.LastCollidedAttributes`))))))
    (else
      (`KismetSystemLibrary.PrintString` "Invalid Collision"))))

(event `BallCollision`
  ;[1 1 1] All Possible Responses
  ;; Ball Responses
  (`|ExecutionSequence`
    (:`then_0`
      (`self.General BallCollision`))))

(event `GreyObjectBallCollision`
  ;[1 1 1] All Possible Responses
  ;; Ball Responses
  (`|ExecutionSequence`
    (:`then_0`
      (`self.General GreyObjectballCollision`))))

(event `ObstacleCollision`
  ;[1 1 1] All Possible Responses
  ;; Obstacle Responses
  (`|ExecutionSequence`
    (:`then_0`
      (`self.General ObstacleCollision`))))

(event `WallCollision`
  ;[1 1 1] All Possible Responses
  ;; Obstacle Responses
  (`|ExecutionSequence`
    (:`then_0`
      (`self.General WallCollision`))))

(event `8BallCollision`
  (params (`8Ball Category` :type "GameplayTagContainer Structure"))
  ;[1 1 1] All Possible Responses
  ;; Ball Responses
  (`|ExecutionSequence`
    (:`then_0`
      (`self.General 8BallCollision`))))

(event `CueBallCollision`
  (params (CueballCategory :type "GameplayTagContainer Structure"))
  ;[1 1 1] All Possible Responses
  ;; Ball Responses
  (`|ExecutionSequence`
    (:`then_0`
      (`self.General CueCollision`))))

(event `BumperCollision`
  ;[1 1 1] All Possible Responses
  ;; Obstacle Responses
  (`|ExecutionSequence`
    (:`then_0`
      (`self.General BumperCollision`))))

(event `PlugCollision`
  ;[1 1 1] All Possible Responses
  ;; Obstacle Responses
  (`|ExecutionSequence`
    (:`then_0`
      (`self.General PlugCollision`))))

(event `ObjectBallCollision`
  ;[1 1 1] All Possible Responses
  ;; Ball Responses
  (`|ExecutionSequence`
    (:`then_0`
      (`self.General ObjectballCollision`))))

(event `ColorballCollision`
  (params (`Color Category` :type "GameplayTagContainer Structure"))
  ;[1 1 1] All Possible Responses
  ;; Ball Responses
  (`|ExecutionSequence`
    (:`then_0`
      (`self.General ColorBallCollision`))))

(event `SetActorActivatedState`
  (params (`Actor Active State` :type Boolean))
  (bind (_returnvalue_x _returnvalue_y) (`KismetMathLibrary.BreakVector` (`self.K2_GetActorLocation`)))
  (bind _returnvalue_x_2 (`KismetMathLibrary.BreakVector` (`self.K2_GetActorLocation`)))
  (bind (_returnvalue_x_3 _returnvalue_y_2) (`KismetMathLibrary.BreakVector` (`self.K2_GetActorLocation`)))
  (bind (_returnvalue_x_4 _returnvalue_y_3) (`KismetMathLibrary.BreakVector` (`self.K2_GetActorLocation`)))
  (bind _ball_reactivate_x_offset_base (`self.Ball Reactivate X offset Base`))
  (bind _ball_reactivate_y_offset_base (`self.Ball Reactivate Y offset Base`))
  ; Activestate
  (if `Actor Active State`
    (`|ExecutionSequence`
      (:`then_0`
        (`self.K2_SetActorLocation` (`KismetMathLibrary.MakeVector` (+ (`KismetMathLibrary.SelectFloat` (* _ball_reactivate_x_offset_base -1.0) _ball_reactivate_x_offset_base (> _returnvalue_x_2 0.0)) _returnvalue_x_4) (+ (`KismetMathLibrary.SelectFloat` (* _ball_reactivate_y_offset_base -1.0) _ball_reactivate_y_offset_base (> _returnvalue_y 0.0)) _returnvalue_y_3) (`self.Ball Base Z height`)) false true)))
    (else
      ;; Teleport ball directly down while reducing speed to 0
      (`|ExecutionSequence`
        (:`then_0`
          (`self.SetBallVelocity` (0.0 0.0 0.0)))
        (:`then_1`
          (`self.K2_SetActorLocation` (`KismetMathLibrary.MakeVector` _returnvalue_x_3 _returnvalue_y_2 -10.0) false true))))))

(event `DisableBallsBelowZ`
  (bind (_returnvalue_x _returnvalue_y _returnvalue_z) (`KismetMathLibrary.BreakVector` (`self.K2_GetActorLocation`)))
  (if (< _returnvalue_z (`self.Ball Base Z height`))
    (set `self.Tags` (`|MakeArray` "None" :!type "Name"))
    (else
      (set `self.Tags` (`|MakeArray` "IgnoreCol" :!type "Name")))))

(fn `CollisionHandler`
  (params (CollisionData :type "HitResult Structure") (CollidedObjectData :type "/Game/Blueprints/Balls/S_GameplayAttributes Structure"))
  (locals (CollidedCategory :type "GameplayTagContainer Structure") (`Collided Interaction Tags` :type "GameplayTagContainer Structure"))
  (bind (_name _score _multiplier _weight _money _category _ballclass _price _statetags _interactiontags) (break `/Game/Blueprints/Balls/S_GameplayAttributes` (`local.CollidedObjectData`)))
  ;[1 1 1] Make Local Variable For Category And Interaction Tags, then trigger any collision event
  (set `local.CollidedCategory` _category)
  (bind _output_get (set `local.Collided Interaction Tags` _interactiontags))
  (`self.AnyCollision` _output_get true)
  (`|ExecutionSequence`
    (:`then_0`
      ;[1 1 1] Ball tree
      ;; Check If collided Object is any ball
      (if (`BlueprintGameplayTagLibrary.HasTag` (`local.CollidedCategory`) (struct :`TagName` "Ball"))
        ;; Trigger General Ball response, then check for specifics
        (`self.BallCollision`)
        (`|ExecutionSequence`
          (:`then_0`
            (`|ExecutionSequence`
              (:`then_0`
                ;; Check if collided ball was an object ball, if so trigger general object ball response then move on to next level.
                (if (`BlueprintGameplayTagLibrary.HasTag` (`local.CollidedCategory`) (struct :`TagName` "Ball.ObjectBall"))
                  (`|ExecutionSequence`
                    (:`then_0`
                      (`self.ObjectBallCollision`))
                    (:`then_1`
                      ;; Check id collided Object ball was grey, if so trigger specific grey response
                      (if (`BlueprintGameplayTagLibrary.HasTag` (`local.CollidedCategory`) (struct :`TagName` "Ball.ObjectBall.Grey"))
                        (`self.GreyObjectBallCollision`))))))
              (:`then_1`
                ;; Check if collided ball was a color ball, if so trigger color ball response.
                (if (`BlueprintGameplayTagLibrary.HasTag` (`local.CollidedCategory`) (struct :`TagName` "Ball.ObjectBall.Color"))
                  (`self.ColorballCollision` (`local.CollidedCategory`))))))
          (:`then_1`
            (`|ExecutionSequence`
              (:`then_0`
                ;; Check If ball is a cue ball
                (if (`BlueprintGameplayTagLibrary.HasTag` (`local.CollidedCategory`) (struct :`TagName` "Ball.Cue"))
                  (`self.CueBallCollision` (`local.CollidedCategory`))))
              (:`then_1`
                ;; Check if ball is an 8 Ball
                (if (`BlueprintGameplayTagLibrary.HasTag` (`local.CollidedCategory`) (struct :`TagName` "Ball.8Ball"))
                  (`self.8BallCollision` (`local.CollidedCategory`)))))))))
    (:`then_1`
      ;[1 1 1] Obstacle Tree
      ;; Check If Collided Object Is an obstacle
      (if (`BlueprintGameplayTagLibrary.HasTag` (`.Category_14_16EB49B74E54F76EB6ED01A647D64054` (break `/Game/Blueprints/Balls/S_GameplayAttributes` (`local.CollidedObjectData`))) (struct :`TagName` "Obstacle"))
        ;; Trigger General Obstacle response, then check for specifics
        (`|ExecutionSequence`
          (:`then_0`
            (`|ExecutionSequence`
              (:`then_0`
                ;; Check If obstacle is wall
                (if (`BlueprintGameplayTagLibrary.HasTag` (`local.CollidedCategory`) (struct :`TagName` "Obstacle.Wall"))
                  (`self.WallCollision`)))
              (:`then_1`
                ;; Check If obstacle is plug
                (if (`BlueprintGameplayTagLibrary.HasTag` (`local.CollidedCategory`) (struct :`TagName` "Obstacle.Plug"))
                  (`self.PlugCollision`)))
              (:`then_2`
                ;; Check If obstacle is plug
                (if (`BlueprintGameplayTagLibrary.HasTag` (`local.CollidedCategory`) (struct :`TagName` "Obstacle.Bumper"))
                  (`self.BumperCollision`)))))
          (:`then_1`
            (`self.ObstacleCollision`)))))))

(fn `First AnyCollision`
  (params (`Interaction Payload` :type "GameplayTagContainer Structure"))
  (`|ExecutionSequence`
    (:`then_0`
      ;[1 1 1] Try using interaction payload
      (`self.TryInteract` (`local.Interaction Payload`)))))

(fn `General 8BallCollision`)

(fn `General BallCollision`
  (`|ExecutionSequence`
    (:`then_0`
      (`self.AudioEventBallCollision`))))

(fn `General BumperCollision`)

(fn `General ColorBallCollision`)

(fn `General CueCollision`)

(fn `General GreyObjectballCollision`)

(fn `General ObjectballCollision`)

(fn `General ObstacleCollision`)

(fn `General PlugCollision`)

(fn `General WallCollision`)

(fn `Paint`
  (params (TextureRenderTarget :type "TextureRenderTarget2D Object Reference") (Position :type "Vector Structure") (Erase :type Boolean) (Density :type "Float (double-precision)") (Radius :type "Float (double-precision)") (TargetMesh :type "Actor Object Reference"))
  (bind (_canvas _size _context) (`KismetRenderingLibrary.BeginDrawCanvasToRenderTarget` TextureRenderTarget))
  (set `self.Size` _size)
  (set `self.Context` _context)
  (set `self.Canvas` _canvas)
  (`MaterialInstanceDynamic.SetVectorParameterValue` (`self.PaintMat`) "PaintCenter" (`KismetMathLibrary.Conv_VectorToLinearColor` (/ (`local.Position`) (.z (`.BoxExtent` (`self.GetActorBounds` (`local.TargetMesh`) false false))))))
  (`MaterialInstanceDynamic.SetScalarParameterValue` (`self.PaintMat`) "Density" (`KismetMathLibrary.SelectFloat` -1000.0 (`local.Density`) (`local.Erase`)))
  (`MaterialInstanceDynamic.SetScalarParameterValue` (`self.PaintMat`) "Radius" (/ (`local.Radius`) (.z (`.BoxExtent` (`self.GetActorBounds` (`local.TargetMesh`) false false)))))
  (`Canvas.K2_DrawMaterial` (`self.Canvas`) (`self.PaintMat`) (0.0 0.0) (`self.Size`) (0.0 0.0) (1.0 1.0) 0.0 (0.5 0.5))
  (`KismetRenderingLibrary.EndDrawCanvasToRenderTarget` (`self.Context`)))

(fn `ReturnAllRelevantCollisionData`
  (returns (GameplayAttributes :type "/Game/Blueprints/Balls/S_GameplayAttributes Structure"))
  (return (`self.S_GameplayAttributes`)))

(fn `Triggered`)

(fn `UserConstructionScript`
  (`parent.UserConstructionScript`))