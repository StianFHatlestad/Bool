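; BP_Cueball is the cue ball Blueprint, whose only active logic is the visual effect for being pocketed.
; PlayPocketEffect spawns the NS_BallPotBasic Niagara system at the ball's location.
; It feeds the system the pocketed hole's XY at a fixed height, the normalized 2D ball velocity and the ball material.
; The velocity direction is also printed to screen as debug output.
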(event `self.ReceiveTick`
  (params (DeltaSeconds :type "Float (single-precision)")))

(event `self.PlayPocketEffect`
  (params (PocketID :type Integer) (PocketActor :type "/Game/Blueprints/Core/BP_Pocket Object Reference"))
  (bind _returnvalue (`KismetMathLibrary.Vector_Normal2D` (`self.GetBallVelocity`)))
  (bind _returnvalue_2 (`NiagaraFunctionLibrary.SpawnSystemAtLocation` "/Game/VFX/Niagara/Systems/PottingEffects/NS_BallPotBasic.NS_BallPotBasic" (`self.K2_GetActorLocation`)))
  (`|ExecutionSequence`
    (:`then_0`
      (`NiagaraComponent.SetVariablePosition` _returnvalue_2 "Pocket" (`KismetMathLibrary.MakeVector` (.x (`self.K2_GetActorLocation` (`self.PocketedHole`))) (.y (`self.K2_GetActorLocation` (`self.PocketedHole`))) -20.0)))
    (:`then_1`
      (`NiagaraComponent.SetVariableVec3` _returnvalue_2 "VelForward" _returnvalue)
      (`KismetSystemLibrary.PrintString` (`KismetStringLibrary.Conv_VectorToString` _returnvalue)))
    (:`then_2`
      (`NiagaraComponent.SetVariableMaterial` _returnvalue_2 "Ballmat" (`self.BallMat`)))))

(fn `UserConstructionScript`)