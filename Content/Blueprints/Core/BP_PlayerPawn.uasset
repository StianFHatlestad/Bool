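; Player pawn for a billiards game, handling cue stick, camera zoom, aim preview and debug keys for test shots and round control.
; Tick derives aiming, waiting and charging gameplay tags from shot state and feeds charge strength to a UI parameter collection.
; Niagara aim lines use sphere traces and the physics solver, temporarily overriding cue ball velocity to predict bounces.
; Shots play a cue montage whose notify hides the stick and plays strength-based sound.
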(event `self.ReceiveBeginPlay`
  (`|ExecutionSequence`
    (:`then_0`
      (`self.InitCamera`))))

(event `/Game/Blueprints/Core/Interfaces/BPI_RoundBasedActors.SpawnCueStick`
  ;[1 1 1] SpawnCue
  (`|ExecutionSequence`
    (:`then_0`
      (bind _outactors (`GameplayStatics.GetAllActorsOfClass` "/Game/Blueprints/Balls/BP_Ball.BP_Ball_C"))
      (for _array_element _outactors
        (if (`self.ActorHasTag` _array_element "CueBallTag")
          (set `self.CueBall` _array_element))))
    (:`then_1`
      (`KismetSystemLibrary.DelayUntilNextTick`)
      (bind _returnvalue (`|SpawnActorFromClass` "/Game/Blueprints/Core/BP_CuePoleActor.BP_CuePoleActor_C" (`KismetMathLibrary.MakeTransform` (`self.K2_GetActorLocation` (`self.CueBall`))) "Undefined" "MultiplyWithRoot" null null))
      (set `self.CueStick` _returnvalue))))

(event `/Game/Blueprints/Core/Interfaces/BPI_RoundBasedActors.DestroyCueStick`
  ;[1 1 1] DestroyCue
  (`self.K2_DestroyActor` (`self.CueStick`)))

(event `self.ReceiveTick`
  (params (DeltaSeconds :type "Float (single-precision)"))
  ;[1 1 1] Comment
  (`|ExecutionSequence`
    (:`then_0`
      (`self.DrawBoolPlayerDebugArrows`))
    (:`then_1`
      (if (`self.CanShoot`)
        (`BlueprintGameplayTagLibrary.AddGameplayTag` (`self.PlayerRoundStateTag`) (struct :`TagName` "Player.Game.Aiming"))
        (`BlueprintGameplayTagLibrary.RemoveGameplayTag` (`self.PlayerRoundStateTag`) (struct :`TagName` "Player.Game.WaitingForNextShot"))
        (elif (`self.bCanPlay`)
          (`BlueprintGameplayTagLibrary.AddGameplayTag` (`self.PlayerRoundStateTag`) (struct :`TagName` "Player.Game.WaitingForNextShot"))
          (`BlueprintGameplayTagLibrary.RemoveGameplayTag` (`self.PlayerRoundStateTag`) (struct :`TagName` "Player.Game.Aiming"))
          (else
            (for _array_element (`BlueprintGameplayTagLibrary.BreakGameplayTagContainer` (`self.PlayerRoundStateTag`))
              (`BlueprintGameplayTagLibrary.RemoveGameplayTag` (`self.PlayerRoundStateTag`) _array_element))))))
    (:`then_2`
      (if (`self.bLockedShotTrajectory`)
        (`BlueprintGameplayTagLibrary.AddGameplayTag` (`self.PlayerRoundStateTag`) (struct :`TagName` "Player.Game.Charging"))
        (`BlueprintGameplayTagLibrary.RemoveGameplayTag` (`self.PlayerRoundStateTag`) (struct :`TagName` "Player.Game.Aiming"))
        (`KismetMaterialLibrary.SetScalarParameterValue` "/Game/Assets/UI/Materials/MPC_UI.MPC_UI" "ShotStrenght" (/ (- (`self.CurrentShotStrength`) 100.0) (- (`self.MaxShootingSpeed`) 100.0)))
        (else
          (`BlueprintGameplayTagLibrary.RemoveGameplayTag` (`self.PlayerRoundStateTag`) (struct :`TagName` "Player.Game.Charging")))))))

(event `Key|One`
  (params (Key :type "Key Structure"))
  ;[1 1 1] Comment
  (:`Pressed`
    (`self.ShootCueBallAtPosition` (100.0 0.0 0.0))))

(event `self.OnCueBallShotBP`
  ;[1 1 1] BallShot Events
  (`|ExecutionSequence`
    (:`then_0`
      (`|PlayMontage` (`/Game/Blueprints/Core/BP_CuePoleActor.CueMesh` (`self.CueStick`)) "/Game/Assets/Cue/SKM_CueRigTest_Skeleton_Montage.SKM_CueRigTest_Skeleton_Montage"
        (:`then`
          (set `/Game/Blueprints/Core/BP_CuePoleActor.StartedFire` true (`self.CueStick`)))
        (:`OnNotifyBegin`
          (`/Game/Blueprints/Core/BP_CuePoleActor.SetVisibility` (`self.CueStick`) false)
          (set `/Game/Blueprints/Core/BP_CuePoleActor.HasFired` true (`self.CueStick`))
          (if (> (`self.CurrentShotStrength`) 300.0)
            (if (> (`self.CurrentShotStrength`) 800.0)
              (`GameplayStatics.PlaySoundAtLocation` "/Game/SFX/Balls/Shot/Shot_Hard_Cue.Shot_Hard_Cue" (`self.K2_GetActorLocation`) (struct) 1.0 1.0 0.0 null null null null)
              (else
                (`GameplayStatics.PlaySoundAtLocation` "/Game/SFX/Balls/Shot/Shot_Med_Cue.Shot_Med_Cue" (`self.K2_GetActorLocation`) (struct) 1.0 1.0 0.0 null null null null)))
            (else
              (`GameplayStatics.PlaySoundAtLocation` "/Game/SFX/Balls/Shot/Shot_Soft_Cue.Shot_Soft_Cue" (`self.K2_GetActorLocation`) (struct) 1.0 1.0 0.0 null null null null))))))))

(event `EnhancedInput|/Game/Blueprints/Input/InputActions/IA_ShootBall`
  (params (ActionValue :type Boolean) (ElapsedSeconds :type "Float (double-precision)") (TriggeredSeconds :type "Float (double-precision)") (InputAction :type "InputAction Object Reference" :default "/Game/Blueprints/Input/InputActions/IA_ShootBall.IA_ShootBall"))
  ;[1 1 1] BallShot Events
  (:`Triggered`
    (if (`BlueprintGameplayTagLibrary.HasTag` (`self.PlayerRoundStateTag`) (struct :`TagName` "Player.Game.Charging"))
      (`/Engine/EditorBlueprintResources/StandardMacros.DoOnce` false))))

(event `Key|Two`
  (params (Key :type "Key Structure"))
  ;[1 1 1] Comment
  (:`Pressed`
    (`self.ShootCueBallAtPosition` (-100.0 0.0 0.0))))

(event `/Game/Blueprints/Core/Interfaces/BPI_RoundBasedActors.NewTurn`
  ;[1 1 1] BallShot Events
  (`|ExecutionSequence`
    (:`then_0`
      (`self.CueStick`
        (:`then`
          (set `/Game/Blueprints/Core/BP_CuePoleActor.StartedFire` false (`self.CueStick`))
          (set `/Game/Blueprints/Core/BP_CuePoleActor.HasFired` false (`self.CueStick`)))
        (:`else`)))
    (:`then_1`
      (bind _cuestick (`self.CueStick`)
        (:`then`
          (`/Game/Blueprints/Core/BP_CuePoleActor.SetVisibility` _cuestick true))
        (:`else`)))))

(event `Key|Three`
  (params (Key :type "Key Structure"))
  ;[1 1 1] Comment
  (:`Pressed`
    (`self.ShootCueBallAtPosition` (0.0 100.0 0.0))))

(event `Key|Four`
  (params (Key :type "Key Structure"))
  ;[1 1 1] Comment
  (:`Pressed`
    (`self.ShootCueBallAtPosition` (0.0 -100.0 0.0))))

(event `Key|Five`
  (params (Key :type "Key Structure"))
  ;[1 1 1] Comment
  (:`Pressed`
    (bind _asbp_game_instance (cast `/Game/Blueprints/Core/BP_GameInstance` (`GameplayStatics.GetGameInstance`)))
    (`/Game/Blueprints/Core/BP_GameInstance.New round` _asbp_game_instance)))

(event `Key|Zero`
  (params (Key :type "Key Structure"))
  ;[1 1 1] Comment
  (:`Pressed`
    (bind _asbp_game_instance (cast `/Game/Blueprints/Core/BP_GameInstance` (`GameplayStatics.GetGameInstance`)))
    (`/Game/Blueprints/Core/BP_GameInstance.End Round` _asbp_game_instance)))

(event `Key|Six`
  (params (Key :type "Key Structure"))
  ;[1 1 1] Comment
  (:`Pressed`
    (bind _asbp_game_instance (cast `/Game/Blueprints/Core/BP_GameInstance` (`GameplayStatics.GetGameInstance`)))
    (set `BoolGameInstance.PlayerGold` 100 _asbp_game_instance)))

(event `Key|MouseScrollUp`
  (params (Key :type "Key Structure"))
  ;[1 1 1] zoom in
  (:`Pressed`
    (set `self.CamZOffsetValue` (- (`self.CamZOffsetValue`) (`self.Zoom`)))))

(event `Key|MouseScrollDown`
  (params (Key :type "Key Structure"))
  ;[1 1 1] zoom out
  (:`Pressed`
    (set `self.CamZOffsetValue` (+ (`self.CamZOffsetValue`) (`self.Zoom`)))))

(event `InitCamera`
  ;[1 1 1] StartCam
  (`|ExecutionSequence`
    (:`then_0`
      (bind _asbp_bool_camera_manager (cast `/Game/Blueprints/Core/Bp_BoolCameraManager` (`GameplayStatics.GetPlayerCameraManager` 0)))
      (set `self.CameraManager` _asbp_bool_camera_manager))))

(fn `DrawBoolPlayerDebugArrows`
  (locals (`Cue Ball Location` :type "Vector Structure" :default (0.0 0.0 0.0)) (`Aim To Cue Dir` :type "Vector Structure" :default (0.0 0.0 0.0)) (CueScaledRadius :type "Float (double-precision)") (OldVelCueBall :type "Vector Structure" :default (0.0 0.0 0.0)) (InitialArrowDrawDist :type "Float (double-precision)" :default 0.0))
  (bind _cueball (`self.CueBall`))
  (bind _cueball_2 (`self.CueBall`))
  (bind _ns_aiminglinebounces (`self.NS_AimingLineBounces`))
  (bind _ns_aiminglinebounces_2 (`self.NS_AimingLineBounces`))
  (bind _returnvalue (`SphereComponent.GetScaledSphereRadius` (`BallActor.SphereComponent` (`self.CueBall`))))
  (bind _returnvalue_2 (`SphereComponent.GetScaledSphereRadius` (`BallActor.SphereComponent` (`self.CueBall`))))
  (`/Engine/EditorBlueprintResources/StandardMacros.IsValid` (`self.CueBall`)
    (:`Is Valid`
      (set `local.Cue Ball Location` (`self.K2_GetActorLocation` (`self.CueBall`)))
      (set `local.CueScaledRadius` (`SphereComponent.GetScaledSphereRadius` (`BallActor.SphereComponent` (`self.CueBall`))))
      (if (`self.CanShoot`)
        (`SceneComponent.SetVisibility` (`self.NS_aimingLine`) true false)
        (set `local.InitialArrowDrawDist` (`KismetMathLibrary.Vector_Distance` (`self.AimLocation`) (`local.Cue Ball Location`)))
        (set `local.OldVelCueBall` (`BallActor.GetBallVelocity` (`self.CueBall`)))
        (`BallActor.SetBallVelocity` (`self.CueBall`) (* (`self.FireDir`) (+ (`KismetMathLibrary.Vector_Distance` (`self.AimLocation`) (`local.Cue Ball Location`)) (`SphereComponent.GetScaledSphereRadius` (`BallActor.SphereComponent` (`self.CueBall`))))))
        (bind (_outhit _returnvalue_3) (`KismetSystemLibrary.SphereTraceSingleForObjects` (`local.Cue Ball Location`) (+ (* (`self.FireDir`) (+ (`KismetMathLibrary.Vector_Distance` (`self.AimLocation`) (`local.Cue Ball Location`)) _returnvalue_2)) (`local.Cue Ball Location`)) _returnvalue_2 (`|MakeArray` "ObjectTypeQuery10" :!type "EObjectTypeQuery Enum") false (`|MakeArray` (`self.CueBall`) :!type "Actor Object Reference")))
        (if _returnvalue_3
          (`SceneComponent.SetVisibility` (`self.NS_AimingRing`) true false)
          (bind _returnvalue_4 (`PhysicsSolverBlueprintBase.OtherBallCollisionSetExitDirection` (`BallActor.PhysicsSolver` _cueball_2) (`|MakeArray` _cueball_2) (cast `BallActor` (`.HitActor` (`GameplayStatics.BreakHitResult` _outhit)) :!pure true) _cueball_2 (0.0 0.0 0.0) _outhit))
          (bind (_bblockinghit _binitialoverlap _time _distance _location _impactpoint _normal _impactnormal _physmat _hitactor) (`GameplayStatics.BreakHitResult` _outhit))
          (bind _returnvalue_5 (`PhysicsSolverBlueprintBase.BallCollisionSetExitDirection` (`BallActor.PhysicsSolver` _cueball) _cueball (`|MakeArray` (cast `BallActor` _hitactor :!pure true)) _outhit))
          (else
            (`BallActor.SetBallVelocity` (`self.CueBall`) (`local.OldVelCueBall`))))
        (`|ExecutionSequence`
          (:`then_0`
            (bind (_outhit_2 _returnvalue_6) (`KismetSystemLibrary.SphereTraceSingle` (`local.Cue Ball Location`) (+ (* (`self.FireDir`) (+ (`KismetMathLibrary.Vector_Distance` (`self.AimLocation`) (`local.Cue Ball Location`)) _returnvalue)) (`local.Cue Ball Location`)) _returnvalue "TraceTypeQuery1" false (`|MakeArray` (`self.CueBall`) :!type "Actor Object Reference")))
            (if _returnvalue_6
              (bind (_bblockinghit_2 _binitialoverlap_2 _time_2 _distance_2 _location_2) (`GameplayStatics.BreakHitResult` _outhit_2))
              (set `local.InitialArrowDrawDist` (`KismetMathLibrary.Vector_Distance` _location_2 (`local.Cue Ball Location`)))
              (`SceneComponent.SetVisibility` (`self.NS_AimingRing`) true false)
              (`NiagaraComponent.SetVariableVec3` (`self.NS_AimingRing`) "RingPos" _location_2)
              (else
                (`SceneComponent.SetVisibility` (`self.NS_AimingRing`) false false))))
          (:`then_1`
            (`|ExecutionSequence`
              (:`then_0`
                (`NiagaraComponent.SetVariableVec3` (`self.NS_aimingLine`) "MainLineStart" (`local.Cue Ball Location`)))
              (:`then_1`
                (`NiagaraComponent.SetVariableVec3` (`self.NS_aimingLine`) "MainLineEnd" (+ (* (`self.FireDir`) (`local.InitialArrowDrawDist`)) (`local.Cue Ball Location`))))
              (:`then_2`
                (if _bblockinghit
                  (`SceneComponent.SetVisibility` (`self.NS_AimingLineBounces`) true false)
                  (`|ExecutionSequence`
                    (:`then_0`
                      (bind _returnvalue_7 (`self.K2_GetActorLocation` _hitactor))
                      (`NiagaraComponent.SetVariableVec3` _ns_aiminglinebounces_2 "LineOneStart" _returnvalue_7))
                    (:`then_1`
                      (`NiagaraComponent.SetVariableVec3` _ns_aiminglinebounces_2 "LineOneEnd" (+ _returnvalue_7 (* _returnvalue_4 (`self.SecondDebugArrowLength`)))))
                    (:`then_2`
                      (`|ExecutionSequence`
                        (:`then_0`
                          (`NiagaraComponent.SetVariableVec3` _ns_aiminglinebounces "LineTwoStart" _location))
                        (:`then_1`
                          (`NiagaraComponent.SetVariableVec3` _ns_aiminglinebounces "LineTwoEnd" (+ _location (* _returnvalue_5 (`self.SecondDebugArrowLength`)))))
                        (:`then_2`
                          (`|ExecutionSequence`
                            (:`then_0`
                              (`NiagaraComponent.SetVariableVec3` (`self.NS_AimingRing`) "RingPos" (`self.K2_GetActorLocation` _hitactor)))
                            (:`then_1`
                              (`BallActor.SetBallVelocity` (`self.CueBall`) (`local.OldVelCueBall`))))))))
                  (else
                    (`SceneComponent.SetVisibility` (`self.NS_AimingLineBounces`) false false)))))))
        (else
          (`SceneComponent.SetVisibility` (`self.NS_AimingRing`) false false)
          (`SceneComponent.SetVisibility` (`self.NS_aimingLine`) false false)
          (`SceneComponent.SetVisibility` (`self.NS_AimingLineBounces`) false false))))))

(fn `UserConstructionScript`)