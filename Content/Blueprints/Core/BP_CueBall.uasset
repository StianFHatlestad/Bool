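; Cue ball Blueprint that orients its mesh along the ball's velocity and prints debug readouts of speed and physics state.
; Each tick it runs SpeedBuffer, which compares current speed with a buffered value refreshed after a short delay.
; A drop below the buffered speed sets JustCrashed, which is only printed alongside the absolute speed change, with no effects attached.
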(event `self.ReceiveBeginPlay`
  (set `self.BufferSpeed` (`KismetMathLibrary.VSize` (`self.GetBallVelocity`))))

(event `self.ReceiveTick`
  (params (DeltaSeconds :type "Float (single-precision)"))
  (`|ExecutionSequence`
    (:`then_0`
      (`KismetSystemLibrary.PrintString` (`KismetStringLibrary.Concat_StrStr` "CueBall Speed: " (`KismetStringLibrary.Conv_DoubleToString` (* (`KismetMathLibrary.VSize` (`self.GetBallVelocity`)) 0.036)) " km/h") true true (struct :`R` 1.0 :`G` 0.015653 :`A` 1.0) 0.0 "77"))
    (:`then_1`
      ;[1 1 1] Debug statement, remove if bothersome
      (`KismetSystemLibrary.PrintString` (`|GetEnumeratorNameAsString` (`self.PhysicsState`)) true true (struct :`G` 0.66 :`B` 1.0 :`A` 1.0) 0.0))
    (:`then_2`
      (`SceneComponent.K2_SetWorldRotation` (`self.MeshComponent`) (`KismetMathLibrary.MakeRotFromX` (`self.GetBallVelocity`)) false false))
    (:`then_3`
      (`self.SpeedBuffer`))))

(event `SpeedBuffer`
  (`|ExecutionSequence`
    (:`then_0`
      (set `self.CurrentSpeed` (`KismetMathLibrary.VSize` (`self.GetBallVelocity`)))
      (`KismetSystemLibrary.Delay` 0.01)
      (set `self.SpeedDelta` (- (`self.BufferSpeed`) (`self.CurrentSpeed`)))
      (set `self.BufferSpeed` (`KismetMathLibrary.VSize` (`self.GetBallVelocity`))))
    (:`then_1`
      (bind _output_get (set `self.JustCrashed` (< (`self.CurrentSpeed`) (`self.BufferSpeed`))))
      (`KismetSystemLibrary.PrintString` (`KismetStringLibrary.Conv_BoolToString` _output_get) true true (struct :`R` 1.0 :`G` 0.152706 :`A` 1.0) 2.0 "22222"))
    (:`then_2`
      (`KismetSystemLibrary.PrintString` (`KismetStringLibrary.Conv_DoubleToString` (`KismetMathLibrary.Abs` (`self.SpeedDelta`))) true true (struct :`G` 1.0 :`B` 0.497896 :`A` 1.0) 2.0 "d22d2d"))))

(fn `UserConstructionScript`)