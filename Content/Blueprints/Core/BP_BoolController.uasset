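; BP_BoolController is a player controller that tracks the mouse and offers a debug switch to a first-person pawn.
; It caches the BP_PlayerPawn on BeginPlay, then each tick stores and prints the DPI-scaled viewport mouse position, clamped to 0–1.
; IA_Debug possesses BP_FirstPersonBool actors tagged FirstPerson and calls OnPosess.
; The table-camera view switch and mouse-driven camera offset logic are disconnected, leaving OffsetCam empty.
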(event `self.ReceiveBeginPlay`
  (`|ExecutionSequence`
    (:`then_0`
      (bind _asbp_player_pawn (cast `/Game/Blueprints/Core/BP_PlayerPawn` (`GameplayStatics.GetPlayerPawn` 0)))
      (set `self.Boolplayer` _asbp_player_pawn))))

(event `TrackViewportMousePos`
  (bind _returnvalue (`WidgetLayoutLibrary.GetViewportScale`))
  (bind (_returnvalue_x _returnvalue_y) (`KismetMathLibrary.BreakVector2D` (`WidgetLayoutLibrary.GetViewportSize`)))
  (`|ExecutionSequence`
    (:`then_0`
      (bind _returnvalue_2 (`WidgetLayoutLibrary.GetMousePositionOnViewport`))
      (`|ExecutionSequence`
        (:`then_0`
          (set `self.MousePosX` (`KismetMathLibrary.FClamp` (/ (* (`KismetMathLibrary.BreakVector2D` _returnvalue_2) _returnvalue) _returnvalue_x))))
        (:`then_1`
          (set `self.MousePosY` (`KismetMathLibrary.FClamp` (/ (* (`.Y` (`KismetMathLibrary.BreakVector2D` _returnvalue_2)) _returnvalue) _returnvalue_y))))))
    (:`then_1`
      (`KismetSystemLibrary.PrintString` (`KismetStringLibrary.Concat_StrStr` " \n___________ \n \n" (`KismetStringLibrary.Concat_StrStr` "XMousePos: " (`KismetStringLibrary.Conv_DoubleToString` (`self.MousePosX`)) " \n" "YMousePos:  " (`KismetStringLibrary.Conv_DoubleToString` (`self.MousePosY`))) " \n \n____________") true true (struct :`R` 0.853487 :`B` 1.0 :`A` 1.0) 2.0 "Mouse"))))

(event `self.ReceiveTick`
  (params (DeltaSeconds :type "Float (single-precision)"))
  (`|ExecutionSequence`
    (:`then_0`
      (`self.TrackViewportMousePos`))))

(event `EnhancedInput|/Game/Blueprints/Input/InputActions/IA_Debug`
  (params (ActionValue :type Boolean) (ElapsedSeconds :type "Float (double-precision)") (TriggeredSeconds :type "Float (double-precision)") (InputAction :type "InputAction Object Reference" :default "/Game/Blueprints/Input/InputActions/IA_Debug.IA_Debug"))
  (:`Started`
    (bind _outactors (`GameplayStatics.GetAllActorsWithTag` "FirstPerson"))
    (for _array_element _outactors
      (bind _asbp_first_person_bool (cast `/Game/Blueprints/Core/BP_FirstPersonBool` _array_element :!pure true))
      (`self.Possess` _asbp_first_person_bool)
      (`/Game/Blueprints/Core/BP_FirstPersonBool.OnPosess` _asbp_first_person_bool))))

(event `OffsetCam`
  ;[1 1 1] Offset
)

(fn `UserConstructionScript`)