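; BP_ObjectRework is a numbered, colored ball actor, apparently a billiard-style ball, with a mesh and a sphere collision component.
; Its construction script creates a dynamic instance of MM_Ballmat and feeds BallNumber and BallColor into the Number and Basetype scalar parameters, so one material covers each ball variant.
; The sphere's overlap and hit events are empty, with disconnected debug print and draw-sphere nodes left in the graph.
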(event `self.SphereComponent.OnComponentBeginOverlap`
  (params (OverlappedComponent :type "PrimitiveComponent Object Reference") (OtherActor :type "Actor Object Reference") (OtherComp :type "PrimitiveComponent Object Reference") (OtherBodyIndex :type Integer) (bFromSweep :type Boolean) (SweepResult :type "HitResult Structure (by ref)")))

(event `self.SphereComponent.OnComponentHit`
  (params (HitComponent :type "PrimitiveComponent Object Reference") (OtherActor :type "Actor Object Reference") (OtherComp :type "PrimitiveComponent Object Reference") (NormalImpulse :type "Vector Structure") (Hit :type "HitResult Structure (by ref)")))

(fn `UserConstructionScript`
  (`parent.UserConstructionScript`)
  (bind _returnvalue (`PrimitiveComponent.CreateDynamicMaterialInstance` (`self.MeshComponent`) 0 "/Game/Materials/Balls/MM_Ballmat.MM_Ballmat" "None"))
  (set `self.BallMat` _returnvalue)
  (`|ExecutionSequence`
    (:`then_0`
      (`MaterialInstanceDynamic.SetScalarParameterValue` (`self.BallMat`) "Number" (`KismetMathLibrary.Conv_IntToDouble` (`self.BallNumber`))))
    (:`then_1`
      (`MaterialInstanceDynamic.SetScalarParameterValue` (`self.BallMat`) "Basetype" (`KismetMathLibrary.Conv_IntToDouble` (`self.BallColor`))))))