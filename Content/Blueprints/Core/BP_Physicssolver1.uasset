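; Custom ball physics solver that supplies exit direction and speed, linear and angular, for ball-ball and ball-wall collisions.
; Directions blend the contact axis with its perpendicular, weighted by float curves over normalized dot products; linear directions are flattened to XY.
; Speeds come from multipliers or constants.
; UpdateBallVelocity classifies each ball as rolling, sliding, spinning or stationary, applies that state's friction curve and zeroes velocity below a sleep threshold.
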(fn `BallCollisionSetAngularExitDirection`
  (params (SuggestedAngularVel :type "Vector Structure") (UnModifiedBall :type "BallActor Object Reference") (OtherBallActor :type "BallActor Object Reference") (Hit :type "HitResult Structure (by ref)"))
  (returns (ReturnValue :type "Vector Structure"))
  (locals (OutPutVec :type "Vector Structure") (ParallellDir :type "Vector Structure") (TotalVelLength :type "Float (double-precision)") (FloatCurveValue :type "Float (single-precision)") (DeltaCenters :type "Vector Structure") (DelCentBallVel_AngVelDelCent :type "CurveFloat Object Reference" :default "/Script/Engine.CurveFloat'/Game/Curves/BallCollisions/DelCentBallVel_AngDelCent.DelCentBallVel_AngDelCent'"))
  (bind _output (`self.VectorArrayGetMax` (`|MakeArray` (`BallActor.GetBallVelocity` (`local.UnModifiedBall`)) (`BallActor.GetBallVelocity` (`local.OtherBallActor`)))))
  (bind _floatcurveval (`self.GetNormDotProdFloatCurveVal` (`local.DelCentBallVel_AngVelDelCent`) (`local.DeltaCenters`) _output))
  (set `local.TotalVelLength` (`self.GetCombinedBallVelLength` (`local.UnModifiedBall`) (`local.OtherBallActor`)))
  (bind _output_get (set `local.DeltaCenters` (`self.GetDeltaCenters` (`local.UnModifiedBall`) (`local.OtherBallActor`))))
  (set `local.FloatCurveValue` _floatcurveval)
  (set `local.ParallellDir` (`self.GetParallellDir` _output_get _output true))
  (set `local.OutPutVec` (* (`local.DeltaCenters`) (* (`local.TotalVelLength`) _floatcurveval)))
  (bind _output_get_2 (set `local.OutPutVec` (+ (`local.OutPutVec`) (* (`local.ParallellDir`) (* (`local.TotalVelLength`) (- 1.0 (`local.FloatCurveValue`)))))))
  (return _output_get_2))

(fn `BallCollisionSetAngularExitSpeed`
  (params (SuggestedAngularVel :type "Vector Structure") (UnModifiedBall :type "BallActor Object Reference") (OtherBallActor :type "BallActor Object Reference") (OutDirection :type "Vector Structure") (Hit :type "HitResult Structure (by ref)"))
  (returns (ReturnValue :type "Float (single-precision)"))
  (return 1.0))

(fn `BallCollisionSetExitDirection`
  (params (SuggestedVelocity :type "Vector Structure") (UnModifiedBall :type "BallActor Object Reference") (OtherBallActor :type "BallActor Object Reference") (Hit :type "HitResult Structure (by ref)"))
  (returns (ReturnValue :type "Vector Structure"))
  (locals (OutPutVec :type "Vector Structure") (ParallellDir :type "Vector Structure" :default (0.0 0.0 0.0)) (DelCentBallVel_RevDeltaCent :type "CurveFloat Object Reference" :default "/Script/Engine.CurveFloat'/Game/Curves/BallCollisions/DelCentBallVel_RevDeltaCent.DelCentBallVel_RevDeltaCent'") (DeltaCenters :type "Vector Structure" :default (0.0 0.0 0.0)) (TotalVelLength :type "Float (double-precision)") (FloatCurveValue :type "Float (single-precision)" :default 0.0))
  (bind _output (`self.VectorArrayGetMax` (`|MakeArray` (`BallActor.GetBallVelocity` (`local.UnModifiedBall`)) (`BallActor.GetBallVelocity` (`local.UnModifiedBall`)))))
  (bind _floatcurveval (`self.GetNormDotProdFloatCurveVal` (`local.DelCentBallVel_RevDeltaCent`) (`local.DeltaCenters`) _output))
  (`KismetSystemLibrary.PrintString` null)
  (set `local.TotalVelLength` (`self.GetCombinedBallVelLength` (`local.UnModifiedBall`) (`local.OtherBallActor`)))
  ;[1 1 1] Delta center is WRONG
  (bind _output_get (set `local.DeltaCenters` (`KismetMathLibrary.Normal` (- (`.ImpactPoint` (`GameplayStatics.BreakHitResult` (`local.Hit`))) (`Actor.K2_GetActorLocation` (`local.UnModifiedBall`))))))
  (set `local.FloatCurveValue` _floatcurveval)
  (set `local.ParallellDir` (`self.GetParallellDir` _output_get _output true))
  (set `local.OutPutVec` (* (`local.DeltaCenters`) (* (`local.TotalVelLength`) _floatcurveval)))
  (bind _output_get_2 (set `local.OutPutVec` (+ (`local.OutPutVec`) (* (`local.ParallellDir`) (* (`local.TotalVelLength`) (- 1.0 (`local.FloatCurveValue`)))))))
  (bind _output_get_3 (set `local.OutPutVec` (`KismetMathLibrary.MakeVector` (.x _output_get_2) (.y _output_get_2))))
  (return (`KismetMathLibrary.Normal` _output_get_3)))

(fn `BallCollisionSetExitSpeed`
  (params (SuggestedVelocity :type "Vector Structure") (UnModifiedBall :type "BallActor Object Reference") (OtherBallActor :type "BallActor Object Reference") (OutDirection :type "Vector Structure") (Hit :type "HitResult Structure (by ref)"))
  (returns (ReturnValue :type "Float (single-precision)"))
  (return (* (`KismetMathLibrary.VSize` (`BallActor.GetBallVelocity` UnModifiedBall)) (`self.BallColMultiplier`))))

(fn `DebugCheckBallActors`
  (params (SphereName :type String) (Ball :type "BallActor Object Reference") (OutVelocity :type "Vector Structure"))
  (returns (Matching :type Boolean))
  (return (and (`KismetStringLibrary.EqualEqual_StrStr` (`KismetSystemLibrary.GetDisplayName` (`local.Ball`)) (`local.SphereName`)) (< (`KismetMathLibrary.VSize` (`local.OutVelocity`)) 10.0))))

(fn `GetCombinedBallVelLength`
  (params (Ball1 :type "BallActor Object Reference") (Ball2 :type "BallActor Object Reference"))
  (returns (Output :type "Float (double-precision)"))
  (return (+ (`KismetMathLibrary.VSize` (`BallActor.GetBallVelocity` Ball1)) (`KismetMathLibrary.VSize` (`BallActor.GetBallVelocity` Ball2)))))

(fn `GetDeltaCenters`
  (params (Ball1 :type "Actor Object Reference") (Ball2 :type "Actor Object Reference"))
  (returns (Output :type "Vector Structure"))
  (return (`KismetMathLibrary.Normal` (- (`Actor.K2_GetActorLocation` Ball1) (`Actor.K2_GetActorLocation` Ball2)))))

(fn `GetNormDotProdFloatCurveVal`
  (params (`Float Curve` :type "CurveFloat Object Reference") (Input1 :type "Vector Structure") (Input2 :type "Vector Structure"))
  (returns (FloatCurveVal :type "Float (single-precision)"))
  (return (`CurveFloat.GetFloatValue` (`local.Float Curve`) (`KismetMathLibrary.Dot_VectorVector` (`KismetMathLibrary.Normal` Input1) (`KismetMathLibrary.Normal` Input2)))))

(fn `GetParallellDir`
  (params (Input :type "Vector Structure") (BallVel :type "Vector Structure") (EnableDirCheck :type Boolean))
  (returns (Dir :type "Vector Structure"))
  (locals (OutDir :type "Vector Structure" :default (0.0 0.0 0.0)))
  (bind _returnvalue (`KismetMathLibrary.Normal` (`local.BallVel`)))
  (bind _returnvalue_2 (`KismetMathLibrary.Normal` (`KismetMathLibrary.Cross_VectorVector` (`KismetMathLibrary.Normal` Input) (0.0 0.0 1.0))))
  (set `local.OutDir` _returnvalue_2)
  (if (`local.EnableDirCheck`)
    (if (< (`KismetMathLibrary.Dot_VectorVector` _returnvalue_2 _returnvalue) (`KismetMathLibrary.Dot_VectorVector` _returnvalue (* _returnvalue_2 -1.0)))
      (return (* (`local.OutDir`) -1.0))
      (else
        _)))
  (return (`local.OutDir`)))

(fn `OtherBallCollisionSetAngularExitDirection`
  (params (SuggestedAngularVel :type "Vector Structure") (OtherBallActor :type "BallActor Object Reference") (UnModifiedBall :type "BallActor Object Reference") (Hit :type "HitResult Structure (by ref)"))
  (returns (ReturnValue :type "Vector Structure"))
  (locals (OutPutVec :type "Vector Structure") (ParallellDir :type "Vector Structure") (FloatCurveVal :type "Float (single-precision)") (DeltaCenters :type "Vector Structure") (TotalVelLength :type "Float (double-precision)") (DelCentBallVel_AngDelCent :type "CurveFloat Object Reference" :default "/Script/Engine.CurveFloat'/Game/Curves/BallCollisions/OtherBallDelCentBallVel_AngDelCent.OtherBallDelCentBallVel_AngDelCent'"))
  (set `local.TotalVelLength` (`self.GetCombinedBallVelLength` (`local.UnModifiedBall`) (`local.OtherBallActor`)))
  (bind _output_get (set `local.DeltaCenters` (`self.GetDeltaCenters` (`local.UnModifiedBall`) (`local.OtherBallActor`))))
  (set `local.FloatCurveVal` (`self.GetNormDotProdFloatCurveVal` (`local.DelCentBallVel_AngDelCent`) (`local.DeltaCenters`) (`self.VectorArrayGetMax` (`|MakeArray` (`BallActor.GetBallVelocity` (`local.UnModifiedBall`)) (`BallActor.GetBallVelocity` (`local.OtherBallActor`))))))
  (set `local.ParallellDir` (`self.GetParallellDir` _output_get))
  (set `local.OutPutVec` (* (* (* (`local.DeltaCenters`) -1.0) (* (`local.TotalVelLength`) (`local.FloatCurveVal`))) -1.0))
  (bind _output_get_2 (set `local.OutPutVec` (+ (`local.OutPutVec`) (* (`local.ParallellDir`) (* (`local.TotalVelLength`) (- 1.0 (`local.FloatCurveVal`)))))))
  (return _output_get_2))

(fn `OtherBallCollisionSetAngularExitSpeed`
  (params (SuggestedAngularVel :type "Vector Structure") (OtherBallActor :type "BallActor Object Reference") (UnModifiedBall :type "BallActor Object Reference") (OutDirection :type "Vector Structure") (Hit :type "HitResult Structure (by ref)"))
  (returns (ReturnValue :type "Float (single-precision)"))
  (return 1.0))

(fn `OtherBallCollisionSetExitDirection`
  (params (OtherBallSuggestedVelocity :type "Vector Structure") (OtherBallActor :type "BallActor Object Reference") (UnModifiedBall :type "BallActor Object Reference") (Hit :type "HitResult Structure (by ref)"))
  (returns (ReturnValue :type "Vector Structure"))
  (locals (TotalVelLength :type "Float (double-precision)") (DeltaCenters :type "Vector Structure") (ParallellDir :type "Vector Structure") (OutPutVec :type "Vector Structure") (DelCentBallVel_RevDeltaCent :type "CurveFloat Object Reference" :default "/Script/Engine.CurveFloat'/Game/Curves/BallCollisions/OtherBallDelCentBallVel_RevDeltaCent.OtherBallDelCentBallVel_RevDeltaCent'") (FloatCurveVal :type "Float (single-precision)" :default 0.0))
  (set `local.TotalVelLength` (`self.GetCombinedBallVelLength` (`local.UnModifiedBall`) (`local.OtherBallActor`)))
  ;[1 1 1] FEIL NAVN LOL
  (bind _output_get (set `local.DeltaCenters` (`KismetMathLibrary.Normal` (- (`.ImpactPoint` (`GameplayStatics.BreakHitResult` (`local.Hit`))) (`Actor.K2_GetActorLocation` (`local.OtherBallActor`))))))
  (set `local.FloatCurveVal` (`self.GetNormDotProdFloatCurveVal` (`local.DelCentBallVel_RevDeltaCent`) (`local.DeltaCenters`) (`self.VectorArrayGetMax` (`|MakeArray` (`BallActor.GetBallVelocity` (`local.UnModifiedBall`)) (`BallActor.GetBallVelocity` (`local.OtherBallActor`))))))
  (set `local.ParallellDir` (`self.GetParallellDir` _output_get))
  (set `local.OutPutVec` (* (* (* (`local.DeltaCenters`) -1.0) (* (`local.TotalVelLength`) (`local.FloatCurveVal`))) -1.0))
  (bind _output_get_2 (set `local.OutPutVec` (+ (`local.OutPutVec`) (* (`local.ParallellDir`) (* (`local.TotalVelLength`) (- 1.0 (`local.FloatCurveVal`)))))))
  (bind _output_get_3 (set `local.OutPutVec` (`KismetMathLibrary.MakeVector` (.x _output_get_2) (.y _output_get_2))))
  (return (`KismetMathLibrary.Normal` _output_get_3)))

(fn `OtherBallCollisionSetExitSpeed`
  (params (OtherBallSuggestedVelocity :type "Vector Structure") (OtherBallActor :type "BallActor Object Reference") (UnModifiedBall :type "BallActor Object Reference") (OutDirection :type "Vector Structure") (Hit :type "HitResult Structure (by ref)"))
  (returns (ReturnValue :type "Float (single-precision)"))
  (return (* (`KismetMathLibrary.VSize` (`BallActor.GetBallVelocity` OtherBallActor)) (`self.OtherBallColMultiplier`))))

(fn `UpdateBallVelocity`
  (params (BallActor :type "BallActor Object Reference") (DeltaTime :type "Float (single-precision)"))
  (locals (FrictionCurve :type "CurveFloat Object Reference" :default "/Script/Engine.CurveFloat'/Game/Curves/Friction/RollingBallFriction.RollingBallFriction'") (FrictionCurveVal :type "Float (single-precision)" :default 0.0))
  (`|ExecutionSequence`
    (:`then_0`
      (`self.BallStateSwitch` (`local.BallActor`)
        (:`Rolling`
          (set `local.FrictionCurve` "/Game/Curves/Friction/RollingBallFriction.RollingBallFriction")
          (`BallActor.SetBoolPhysicsState` (`local.BallActor`) "Ebps_Rolling"))
        (:`Sliding`
          (set `local.FrictionCurve` "/Game/Curves/Friction/SlidingBallFriction.SlidingBallFriction")
          (`BallActor.SetBoolPhysicsState` (`local.BallActor`) "Ebps_Sliding"))
        (:`Spinning`
          (set `local.FrictionCurve` "/Game/Curves/Friction/SpinningBallFriction.SpinningBallFriction")
          (`BallActor.SetBoolPhysicsState` (`local.BallActor`) "Ebps_Spinning"))
        (:`Stationary`
          (set `local.FrictionCurve` "/Game/Curves/Friction/StationaryBallFriction.StationaryBallFriction")
          (`BallActor.SetBoolPhysicsState` (`local.BallActor`) "Ebps_Stationary"))))
    (:`then_1`
      (if (> (`KismetMathLibrary.VSize` (`BallActor.GetBallVelocity` (`local.BallActor`))) (`self.SleepVelocityMin`))
        (set `local.FrictionCurveVal` (`CurveFloat.GetFloatValue` (`local.FrictionCurve`) (`KismetMathLibrary.VSize` (`BallActor.GetBallVelocity` (`local.BallActor`)))))
        (`BallActor.SetBallVelocity` (`local.BallActor`) (- (`BallActor.GetBallVelocity` (`local.BallActor`)) (* (* (`BallActor.GetBallVelocity` (`local.BallActor`)) (`local.FrictionCurveVal`)) (`local.DeltaTime`))))
        (else
          (`BallActor.SetBallVelocity` (`local.BallActor`) (0.0 0.0 0.0)))))))

(fn `VectorArrayGetMax`
  (params (InArray :type "Array of Vector Structure"))
  (returns (Output :type "Vector Structure"))
  (locals (Largest :type "Vector Structure" :default (0.0 0.0 0.0)))
  (for _array_element InArray
    (if (> (`KismetMathLibrary.VSize` _array_element) (`KismetMathLibrary.VSize` (`local.Largest`)))
      (set `local.Largest` _array_element)))
  (return (`local.Largest`)))

(fn `VectorArrayGetMin`
  (params (InArray :type "Array of Vector Structure"))
  (returns (Output :type "Vector Structure"))
  (locals (minimum :type "Vector Structure" :default (9999999999.0 9999999999.0 9999999999.0)))
  (for _array_element InArray
    (if (< (`KismetMathLibrary.VSize` _array_element) (`KismetMathLibrary.VSize` (`local.minimum`)))
      (set `local.minimum` _array_element)))
  (return (`local.minimum`)))

(fn `WallCollisionSetAngularExitDirection`
  (params (SuggestedAngularVel :type "Vector Structure") (UnModifiedBall :type "BallActor Object Reference") (Hit :type "HitResult Structure (by ref)"))
  (returns (ReturnValue :type "Vector Structure"))
  (locals (OutPutVec :type "Vector Structure") (FloatCurveVal :type "Float (double-precision)") (SurfaceParallell :type "Vector Structure") (Ball :type "BallActor Object Reference") (NormalXVelDot_To_ImpNormDir :type "CurveFloat Object Reference" :default "/Script/Engine.CurveFloat'/Game/Curves/WallCollisions/NormalXVelDot_To_AngImpNormDir.NormalXVelDot_To_AngImpNormDir'"))
  (bind _returnvalue (`BallActor.GetBallVelocity` (`local.Ball`)))
  (bind _floatcurveval (`self.GetNormDotProdFloatCurveVal` (`local.NormalXVelDot_To_ImpNormDir`) _returnvalue (`.ImpactNormal` (`GameplayStatics.BreakHitResult` (`local.Hit`)))))
  (set `local.Ball` UnModifiedBall)
  (set `local.SurfaceParallell` (`self.GetParallellDir` (`.ImpactNormal` (`GameplayStatics.BreakHitResult` (`local.Hit`))) (`BallActor.GetBallVelocity` (`local.Ball`)) true))
  (set `local.FloatCurveVal` _floatcurveval)
  (set `local.OutPutVec` (* (* (`KismetMathLibrary.VSize` _returnvalue) _floatcurveval) (`.ImpactNormal` (`GameplayStatics.BreakHitResult` (`local.Hit`)))))
  (bind _output_get (set `local.OutPutVec` (+ (`local.OutPutVec`) (* (`local.SurfaceParallell`) (* (`KismetMathLibrary.VSize` (`BallActor.GetBallVelocity` (`local.Ball`))) (- 1.0 (`local.FloatCurveVal`)))))))
  (return _output_get))

(fn `WallCollisionSetAngularExitSpeed`
  (params (SuggestedAngularVel :type "Vector Structure") (UnModifiedBall :type "BallActor Object Reference") (Hit :type "HitResult Structure (by ref)"))
  (returns (ReturnValue :type "Float (single-precision)"))
  (return 1.0))

(fn `WallCollisionSetExitDirection`
  (params (SuggestedVelocity :type "Vector Structure") (UnModifiedBall :type "BallActor Object Reference") (Hit :type "HitResult Structure (by ref)"))
  (returns (ReturnValue :type "Vector Structure"))
  (locals (NormalXVelDot_To_ImpNormDir :type "CurveFloat Object Reference" :default "/Script/Engine.CurveFloat'/Game/Curves/WallCollisions/NormalXVelDot_To_ImpNormDir.NormalXVelDot_To_ImpNormDir'") (SurfaceParallell :type "Vector Structure") (Ball :type "BallActor Object Reference") (Hit :type "HitResult Structure (by ref)") (OutPutVec :type "Vector Structure") (FloatCurveVal :type "Float (double-precision)"))
  (bind _returnvalue (`BallActor.GetBallVelocity` (`local.Ball`)))
  (bind _floatcurveval (`self.GetNormDotProdFloatCurveVal` (`local.NormalXVelDot_To_ImpNormDir`) _returnvalue (`.ImpactNormal` (`GameplayStatics.BreakHitResult` (`local.Hit`)))))
  (`KismetSystemLibrary.PrintString` null "WALL ")
  (set `local.Ball` UnModifiedBall)
  (set `local.SurfaceParallell` (`self.GetParallellDir` (`.ImpactNormal` (`GameplayStatics.BreakHitResult` (`local.Hit`))) (`BallActor.GetBallVelocity` (`local.Ball`)) true))
  (set `local.FloatCurveVal` _floatcurveval)
  (set `local.OutPutVec` (* (* (`KismetMathLibrary.VSize` _returnvalue) _floatcurveval) (`.ImpactNormal` (`GameplayStatics.BreakHitResult` (`local.Hit`)))))
  (bind _output_get (set `local.OutPutVec` (+ (`local.OutPutVec`) (* (`local.SurfaceParallell`) (* (`KismetMathLibrary.VSize` (`BallActor.GetBallVelocity` (`local.Ball`))) (- 1.0 (`local.FloatCurveVal`)))))))
  (bind _output_get_2 (set `local.OutPutVec` (`KismetMathLibrary.MakeVector` (.x _output_get) (.y _output_get))))
  (return _output_get_2))

(fn `WallCollisionSetExitSpeed`
  (params (SuggestedVelocity :type "Vector Structure") (UnModifiedBall :type "BallActor Object Reference") (Hit :type "HitResult Structure (by ref)"))
  (returns (ReturnValue :type "Float (single-precision)"))
  (return (`self.WallColMultiplier`)))