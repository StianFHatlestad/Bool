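; Cue stick actor that follows the player pawn's cue ball and lines up with its fire direction.
; Each tick it caches the ball location, then interpolates rotation and position, sitting behind the ball at a fixed height.
; StartedFire drops the pull-back offset and switches interp speed, and HasFired freezes movement.
; The power bar widget and AnimBP aim-target update are unwired.
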(event `self.ReceiveBeginPlay`
  (`|ExecutionSequence`
    (:`then_0`
      (`self.InitClasses`))
    (:`then_1`
      (`self.LoadPowerBar`))))

(event `LoadPowerBar`)

(event `InitClasses`
  (`|ExecutionSequence`
    (:`then_0`
      (bind _asbp_player_pawn (cast `/Game/Blueprints/Core/BP_PlayerPawn` (`GameplayStatics.GetPlayerPawn` 0)))
      (set `self.Player` _asbp_player_pawn))
    (:`then_1`
      (bind _asabp_cue_pole (cast `/Game/Assets/Cue/ABP_CuePole` (`SkeletalMeshComponent.GetAnimInstance` (`self.CueMesh`))))
      (set `self.AnimBp` _asabp_cue_pole))
    (:`then_2`
      (`self.SetVisibility` true))
    (:`then_3`
      (set `self.Initialized` true))))

(event `self.ReceiveTick`
  (params (DeltaSeconds :type "Float (single-precision)"))
  (if (`self.Initialized`)
    (`|ExecutionSequence`
      (:`then_0`
        (`self.CueballLocationUpdater`))
      (:`then_1`
        (`self.SetActorRotation`))
      (:`then_2`
        (`self.OffsetLocation`))
      (:`then_3`
        (`/Engine/EditorBlueprintResources/StandardMacros.IsValid` (`self.PowerBar`))))))

(event `SetVisibility`
  (params (bNewVisibility :type Boolean))
  (`SceneComponent.SetVisibility` (`self.CueMesh`) bNewVisibility false))

(event `CueballLocationUpdater`
  (set `self.CueBallLocation` (`self.K2_GetActorLocation` (`PlayerPawn.CueBall` (`self.Player`)))))

(event `OffsetLocation`
  (bind (_clampedradiallocation_x _clampedradiallocation_y) (`KismetMathLibrary.BreakVector` (`self.ClampedRadialLocation`)))
  (`|ExecutionSequence`
    (:`then_0`
      (set `self.ClampedRadialLocation` (+ (`self.CueBallLocation`) (* (* (`PlayerPawn.FireDir` (`self.Player`)) (`KismetMathLibrary.SelectFloat` 0.0 (`self.MaxAimingDistanceFromCueball`) (`self.StartedFire`))) -1))))
    (:`then_1`
      (if (not (`self.HasFired`))
        (`self.K2_SetActorLocation` (`KismetMathLibrary.VInterpTo` (`self.K2_GetActorLocation`) (`KismetMathLibrary.MakeVector` _clampedradiallocation_x _clampedradiallocation_y (`self.VerticalOffset`)) (`GameplayStatics.GetWorldDeltaSeconds`) (`KismetMathLibrary.SelectFloat` 3.0 (`self.CueAimLocationSpeed`) (`self.StartedFire`))))))))

(event `UpdateAnimbp`
  (set `/Game/Assets/Cue/ABP_CuePole.CueAimTarget` (`self.CueBallLocation`) (`self.AnimBp`)))

(event `SetActorRotation`
  (`|ExecutionSequence`
    (:`then_0`
      (if (not (`self.HasFired`))
        (`self.K2_SetActorRotation` (`KismetMathLibrary.RInterpTo` (`self.K2_GetActorRotation`) (`KismetMathLibrary.Conv_VectorToRotator` (`PlayerPawn.FireDir` (`self.Player`))) (`GameplayStatics.GetWorldDeltaSeconds`) (`self.CueAimRotationSpeed`)))))))

(fn `UserConstructionScript`)