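; Player pawn for a cue-ball shooting game, providing debug aim visuals and camera zoom.
; Each tick draws a debug sphere at the mouse's world position and an arrow from the current cue ball pointing away from AimLocation.
; The arrow's length scales with shot speed when the trajectory is locked, otherwise with AimLocation's distance from world origin.
; Mouse wheel moves the camera along world Z, with zoom-in floored at zero.
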(event `self.ReceiveBeginPlay`)

(event `self.ReceiveTick`
  (params (DeltaSeconds :type "Float (single-precision)"))
  (bind _returnvalue (`self.K2_GetActorLocation` (`self.CurrentCueBall`)))
  (bind _returnvalue_2 (`self.K2_GetActorLocation` (`self.CurrentCueBall`)))
  (bind _returnvalue_3 (- (`self.K2_GetActorLocation` (`self.CurrentCueBall`)) (`self.AimLocation`)))
  (bind _returnvalue_4 (`KismetMathLibrary.Normal` _returnvalue_3))
  (bind _returnvalue_5 (`self.GetMouseWorldPosition`))
  (`KismetSystemLibrary.DrawDebugSphere` _returnvalue_5 400.0)
  (if (`self.bLockedShotTrajectory`)
    (`KismetSystemLibrary.DrawDebugArrow` _returnvalue_2 (+ (* _returnvalue_4 (/ (`self.CurrentShotSpeed`) 10.0)) _returnvalue) 100.0)
    (else
      (`KismetSystemLibrary.DrawDebugArrow` _returnvalue_2 (+ (* _returnvalue_4 (`KismetMathLibrary.Vector_Distance` _returnvalue_3 _returnvalue)) (`self.K2_GetActorLocation` (`self.CurrentCueBall`))) 100.0))))

(event `Key|MouseScrollUp`
  (params (Key :type "Key Structure"))
  (bind (_returnvalue_x _returnvalue_y _returnvalue_z) (`KismetMathLibrary.BreakVector` (`SceneComponent.K2_GetComponentLocation` (`self.CameraComponent`))))
  (bind _returnvalue (- _returnvalue_z (`self.Zoom`)))
  (:`Pressed`
    (`SceneComponent.K2_SetWorldLocation` (`self.CameraComponent`) (`KismetMathLibrary.MakeVector` _returnvalue_x _returnvalue_y (`KismetMathLibrary.FClamp` _returnvalue 0.0 _returnvalue)) false true)))

(event `Key|MouseScrollDown`
  (params (Key :type "Key Structure"))
  (bind (_returnvalue_x _returnvalue_y _returnvalue_z) (`KismetMathLibrary.BreakVector` (`SceneComponent.K2_GetComponentLocation` (`self.CameraComponent`))))
  (:`Pressed`
    (`SceneComponent.K2_SetWorldLocation` (`self.CameraComponent`) (`KismetMathLibrary.MakeVector` _returnvalue_x _returnvalue_y (+ _returnvalue_z (`self.Zoom`))) false true)))

(fn `UserConstructionScript`)