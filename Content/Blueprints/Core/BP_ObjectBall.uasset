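; BP_ObjectBall is a numbered object ball whose appearance is set by its BaseType and Number variables.
; The construction script creates a dynamic instance of MI_ObjectBall on MeshComponent and passes both variables to it as scalar parameters, so one material serves every ball variant.
; The event graph holds only disabled placeholder events, so the Blueprint adds no runtime logic.
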(fn `UserConstructionScript`
  (`|ExecutionSequence`
    (:`then_0`
      (bind _returnvalue (`PrimitiveComponent.CreateDynamicMaterialInstance` (`self.MeshComponent`) 0 "/Game/Materials/Balls/MI_ObjectBall.MI_ObjectBall" "None"))
      (set `self.BallMat` _returnvalue))
    (:`then_1`
      (`MaterialInstanceDynamic.SetScalarParameterValue` (`self.BallMat`) "BaseType" (`KismetMathLibrary.Conv_IntToDouble` (`self.BaseType`))))
    (:`then_2`
      (`MaterialInstanceDynamic.SetScalarParameterValue` (`self.BallMat`) "Number" (`KismetMathLibrary.Conv_IntToDouble` (`self.Number`))))))