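; BP_CoreHUD is the central UI hub that shows the game's menus, overlays and pop-ups.
; On BeginPlay it caches the game instance, creates the WBP_GameStack widget, seeds its main stack with the match overlay and sets Game-and-UI input.
; One event per screen pushes that widget class onto the stack, with interactions using a separate pop-up push.
; Despite their Toggle names, these events only push and never close screens.
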(event `self.ReceiveBeginPlay`
  ;[1 1 1] On startup
  (`|ExecutionSequence`
    (:`then_0`
      (bind _asbp_game_instance (cast `/Game/Blueprints/Core/BP_GameInstance` (`GameplayStatics.GetGameInstance`)))
      (set `self.GameInstance` _asbp_game_instance))
    (:`then_1`
      (bind _returnvalue (`|CreateWidget` "/Game/Widget/WBP_GameStack.WBP_GameStack_C"))
      (bind _output_get (set `self.GameStack` _returnvalue))
      (`UserWidget.AddToViewport` _output_get 0)
      (`CommonActivatableWidgetContainerBase.BP_AddWidget` (`/Game/Widget/WBP_GameStack.MainStack` _output_get) "/Game/Widget/WBP_MatchOverlay.WBP_MatchOverlay_C")
      (`WidgetBlueprintLibrary.SetInputMode_GameAndUIEx` (`GameplayStatics.GetPlayerController` 0) _returnvalue "LockOnCapture" false))))

(event `Interaction PopUp Toggle`
  ; PopUp Toggles
  (`/Game/Widget/WBP_GameStack.Push Pop up` (`self.GameStack`) "/Game/Widget/WBP_Interaction_PopUp.WBP_Interaction_PopUp_C"))

(event `MainMenuToggle`
  ;[1 1 1] Game Stack Menu toggles
  (`/Game/Widget/WBP_GameStack.Push Widget` (`self.GameStack`) "/Game/Widget/WBP_MainMenu.WBP_MainMenu_C"))

(event `OptionsToggle`
  ;[1 1 1] Game Stack Menu toggles
  (`/Game/Widget/WBP_GameStack.Push Widget` (`self.GameStack`) "/Game/Widget/WBP_Options.WBP_Options_C"))

(event `MatchOverlayToggle`
  ;[1 1 1] Game Stack Menu toggles
  (`/Game/Widget/WBP_GameStack.Push Widget` (`self.GameStack`) "/Game/Widget/WBP_MatchOverlay.WBP_MatchOverlay_C"))

(event `ShopToggle`
  ;[1 1 1] Game Stack Menu toggles
  (`/Game/Widget/WBP_GameStack.Push Widget` (`self.GameStack`) "/Game/Widget/WBP_ShopInterface.WBP_ShopInterface_C"))

(event `TransitionToggle`
  ;[1 1 1] Game Stack Menu toggles
  (`/Game/Widget/WBP_GameStack.Push Widget` (`self.GameStack`) "/Game/Widget/WBP_Tansition.WBP_Tansition_C"))

(event `GameSettupToggle`
  ;[1 1 1] Game Stack Menu toggles
  (`/Game/Widget/WBP_GameStack.Push Widget` (`self.GameStack`) "/Game/Widget/WBP_GameSetup.WBP_GameSetup_C"))

(event `CreditToggle`
  ;[1 1 1] Game Stack Menu toggles
  (`/Game/Widget/WBP_GameStack.Push Widget` (`self.GameStack`) "/Game/Widget/WBP_Credits.WBP_Credits_C"))

(event `ResultToggle`
  ;[1 1 1] Game Stack Menu toggles
  (`/Game/Widget/WBP_GameStack.Push Widget` (`self.GameStack`) "/Game/Widget/WBP_Result.WBP_Result_C"))

(event `GameOverToggle`
  ;[1 1 1] Game Stack Menu toggles
  (`/Game/Widget/WBP_GameStack.Push Widget` (`self.GameStack`) "/Game/Widget/WBP_GameOver.WBP_GameOver_C"))

(event `LoadoutToggle`
  ;[1 1 1] Game Stack Menu toggles
  (`/Game/Widget/WBP_GameStack.Push Widget` (`self.GameStack`) "/Game/Widget/WBP_Loadaout.WBP_Loadaout_C"))

(event `PauseToggle`
  ;[1 1 1] Game Stack Menu toggles
  (`/Game/Widget/WBP_GameStack.Push Widget` (`self.GameStack`) "/Game/Widget/WBP_Pause.WBP_Pause_C"))

(event `VictoryToggle`
  ;[1 1 1] Game Stack Menu toggles
  (`/Game/Widget/WBP_GameStack.Push Widget` (`self.GameStack`) "/Game/Widget/WBP_Vicory.WBP_Vicory_C"))

(event `DialogueToggle`
  ;[1 1 1] Game Stack Menu toggles
  (`/Game/Widget/WBP_GameStack.Push Widget` (`self.GameStack`) "/Game/Widget/WBP_Dialogue.WBP_Dialogue_C"))

(event `Toggle Bar Overlay`
  ;[1 1 1] Game Stack Menu toggles
  (`/Game/Widget/WBP_GameStack.Push Widget` (`self.GameStack`) "/Game/Widget/WBP_Bar.WBP_Bar_C"))

(fn `UserConstructionScript`)