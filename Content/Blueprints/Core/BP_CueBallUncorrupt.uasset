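; BP_CueBallUncorrupt is a cue ball Blueprint that orients its mesh along its direction of travel when moving fast.
; Each tick, SquashState sets a Stretched flag when speed exceeds a fixed threshold.
; While stretched, the mesh switches to absolute rotation and faces the normalized velocity, otherwise it returns to relative rotation.
; No scaling is applied here, and Tick also prints a constant debug value.
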(event `self.ReceiveTick`
  (params (DeltaSeconds :type "Float (single-precision)"))
  (`self.SquashState`)
  (`KismetSystemLibrary.PrintString` (`KismetStringLibrary.Conv_DoubleToString` 0.0)))

(event `SquashState`
  (bind _meshcomponent (`self.MeshComponent`))
  (`|ExecutionSequence`
    (:`then_0`
      (set `self.Stretched` (> (`KismetMathLibrary.VSize` (`self.GetVelocity`)) 164.0)))
    (:`then_1`
      (if (`self.Stretched`)
        (set `SceneComponent.bAbsoluteRotation` true _meshcomponent)
        (`SceneComponent.K2_SetWorldRotation` _meshcomponent (`KismetMathLibrary.MakeRotFromX` (`KismetMathLibrary.Normal` (`self.GetVelocity`))) false false)
        (else
          (set `SceneComponent.bAbsoluteRotation` false (`self.MeshComponent`)))))))

(fn `UserConstructionScript`)