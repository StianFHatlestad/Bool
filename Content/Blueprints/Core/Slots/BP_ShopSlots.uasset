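; BP_ShopSlots is the shop display actor that shows purchasable balls and items in three slots each.
; It spawns BP_BallShopPreview and BP_Item actors from the GameInstance's shop lists, coloring balls by gameplay tag.
; Round payloads hide the store on round start and reveal it on round end through ball box montages, whose notifies time ball visibility.
; Rerolls play a random montage and rebuild the spawned actors, while purchases destroy the bought one.
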(event `/Game/Blueprints/Core/Interfaces/BPI_RoundBasedActors.StoreRerollVisuals`
  ;[1 1 1] Reroll Visuals
  (bind _notifyname (`|PlayMontage` (`self.SKM_BallBox`) (`KismetArrayLibrary.Array_Random` (`self.RerollAnimations`)))
    (:`then`
      (switch `name` _notifyname
        (:`Reroll`
          (`/Game/Blueprints/Core/Interfaces/BPI_RoundBasedActors.UnloadStoreVisuals` false :!label _label)
          (`/Game/Blueprints/Core/Interfaces/BPI_RoundBasedActors.LoadShopVisuals` false))
        (:`Hide`
          (for _array_element (`self.SpawnedBalls`)
            (`SceneComponent.SetVisibility` (`Actor.RootComponent` _array_element) false true)))))
    (:`OnNotifyBegin`
      (goto _label))))

(event `SpawnBalls`
  ;[1 1 1] Spawn Balls
  (for (_array_element _array_index) (`/Game/Blueprints/Core/BP_GameInstance.ShopBalls` (`self.GameInstance`))
    (set `self.CurrentBallslot` (`|GetArrayItem` (`self.ShopBallSlotArray`) _array_index))
    (set `self.CurrentBallStruct` _array_element)
    (bind _returnvalue (`|SpawnActorFromClass` "/Game/Blueprints/Balls/BP_BallShopPreview.BP_BallShopPreview_C" (`KismetMathLibrary.MakeTransform` (0.0 0.0 0.0)) "Undefined" "MultiplyWithRoot" null null))
    (set `self.CurrentBall` _returnvalue)
    (`|ExecutionSequence`
      (:`then_0`
        (`|SwitchGameplayTag` (`|GetArrayItem` (`BlueprintGameplayTagLibrary.BreakGameplayTagContainer` (`.Category_14_16EB49B74E54F76EB6ED01A647D64054` (break `/Game/Blueprints/Balls/S_GameplayAttributes` (`self.CurrentBallStruct`)))))
          (:`Ball.ObjectBall.Color.Red`
            (set `/Game/Blueprints/Balls/BP_BallShopPreview.BallColor` 3 (`self.CurrentBall`)))
          (:`Ball.ObjectBall.Color.Blue`
            (set `/Game/Blueprints/Balls/BP_BallShopPreview.BallColor` 4 (`self.CurrentBall`)))
          (:`Ball.ObjectBall.Color.Yellow`
            (set `/Game/Blueprints/Balls/BP_BallShopPreview.BallColor` 5 (`self.CurrentBall`)))
          (:`Ball.ObjectBall.Color.Green`
            (set `/Game/Blueprints/Balls/BP_BallShopPreview.BallColor` 7 (`self.CurrentBall`)))))
      (:`then_1`
        (set `/Game/Blueprints/Balls/BP_BallShopPreview.BallNumber` 16 (`self.CurrentBall`)))
      (:`then_2`
        (`/Game/Blueprints/Balls/BP_BallShopPreview.SetVisuals` (`self.CurrentBall`)))
      (:`then_3`
        (`self.K2_AttachToComponent` (`self.CurrentBall`) (`self.CurrentBallslot`) "None" "KeepRelative" "KeepRelative" "KeepRelative" true))
      (:`then_4`
        (`KismetArrayLibrary.Array_Add` (`self.SpawnedBalls`) (`self.CurrentBall`)))
      (:`then_5`
        (`SceneComponent.SetVisibility` (`Actor.RootComponent` (`self.CurrentBall`)) (`self.BallsVisible`) true)))))

(event `SpawnItems`
  ;[1 1 1] Spawn Items
  (for (_array_element _array_index) (`/Game/Blueprints/Core/BP_GameInstance.ShopItems` (`self.GameInstance`))
    (set `self.CurrentItemStruct` _array_element)
    (bind _returnvalue_location (`KismetMathLibrary.BreakTransform` (`SceneComponent.K2_GetComponentToWorld` (`|GetArrayItem` (`self.ShopItemSlotArray`) _array_index))))
    (bind _returnvalue (`|SpawnActorFromClass` "/Game/Blueprints/Items/BP_Item.BP_Item_C" (`KismetMathLibrary.MakeTransform` _returnvalue_location) "Undefined" "OverrideRootScale" null null))
    (set `self.CurrentItem` _returnvalue)
    (`|ExecutionSequence`
      (:`then_0`
        (`/Game/Blueprints/Items/BP_Item.SetParams` (`self.CurrentItem`)))
      (:`then_1`
        (set `/Game/Blueprints/Items/BP_Item.Item` (`self.CurrentItemStruct`) (`self.CurrentItem`)))
      (:`then_2`
        (`/Game/Blueprints/Items/BP_Item.SetParams` (`self.CurrentItem`)))
      (:`then_3`
        (`KismetArrayLibrary.Array_Add` (`self.SpawnedItems`) (`self.CurrentItem`))))))

(event `self.ReceiveBeginPlay`
  ; MakeReferences
  (bind _asbp_game_instance (cast `/Game/Blueprints/Core/BP_GameInstance` (`GameplayStatics.GetGameInstance`)))
  (set `self.GameInstance` _asbp_game_instance))

(event `/Game/Blueprints/Core/Interfaces/BPI_RoundBasedActors.UpdateRoundActors`
  (params (RoundStatePayload :type "GameplayTag Structure"))
  ; Recieve Round Payloads
  (`/Game/Blueprints/Macros/BPML_RoundEval.RecieveRoundPayload` RoundStatePayload
    (:`OnRoundStart`
      (`self.Hide Store`))
    (:`OnRoundEnd`
      (`self.Reveal Store`))))

(event `Hide Store`
  ;[1 1 1] Comment
  (bind _notifyname (`|PlayMontage` (`self.SKM_BallBox`) "/Game/Assets/BallBox/Animations/BallBox_End_Montage.BallBox_End_Montage")
    (:`then`
      (set `self.BallsVisible` false))
    (:`OnCompleted`
      (`SceneComponent.SetVisibility` (`self.SKM_BallBox`) (`self.BallsVisible`) true))
    (:`OnNotifyBegin`
      (if (== _notifyname "Show")
        (for _array_element (`self.SpawnedBalls`)
          (bind _rootcomponent (`Actor.RootComponent` _array_element))
          (`/Engine/EditorBlueprintResources/StandardMacros.IsValid` _rootcomponent
            (:`Is Valid`
              (`SceneComponent.SetVisibility` _rootcomponent (`self.BallsVisible`) true))))))))

(event `Reveal Store`
  ;[1 1 1] RevealStore
  (set `self.BallsVisible` true)
  (bind _notifyname (`|PlayMontage` (`self.SKM_BallBox`) "/Game/Assets/BallBox/Animations/BallBox_StartMontage.BallBox_StartMontage")
    (:`then`
      (`KismetSystemLibrary.Delay` 0.07)
      (`SceneComponent.SetVisibility` (`self.SKM_BallBox`) (`self.BallsVisible`) true))
    (:`OnNotifyBegin`
      (if (== _notifyname "Show")
        (for _array_element (`self.SpawnedBalls`)
          (`SceneComponent.SetVisibility` (`Actor.RootComponent` _array_element) (`self.BallsVisible`) true))))))

(event `/Game/Blueprints/Core/Interfaces/BPI_RoundBasedActors.LoadShopVisuals`
  (params (Rerolled :type Boolean))
  ;[1 1 1] Load
  (if (not Rerolled)
    (`|ExecutionSequence`
      (:`then_0`
        (`self.SpawnBalls`))
      (:`then_1`
        (`self.SpawnItems`)))))

(event `/Game/Blueprints/Core/Interfaces/BPI_RoundBasedActors.UnloadStoreVisuals`
  (params (Rerolled :type Boolean))
  ;[1 1 1] Unload
  (if (not Rerolled)
    (`|ExecutionSequence`
      (:`then_0`
        (for _array_element (`self.SpawnedBalls`)
          (`/Engine/EditorBlueprintResources/StandardMacros.IsValid` _array_element
            (:`Is Valid`
              (`self.K2_DestroyActor` _array_element))))
        (`KismetArrayLibrary.Array_Clear` (`self.SpawnedBalls`)))
      (:`then_1`
        (for _array_element_2 (`self.SpawnedItems`)
          (`/Engine/EditorBlueprintResources/StandardMacros.IsValid` _array_element_2
            (:`Is Valid`
              (`self.K2_DestroyActor` _array_element_2))))
        (`KismetArrayLibrary.Array_Clear` (`self.SpawnedItems`))))))

(event `/Game/Blueprints/Core/Interfaces/BPI_RoundBasedActors.ItemBought`
  (params (`Item Index` :type Integer))
  (bind _output (`|GetArrayItem` (`self.SpawnedItems`) `Item Index`))
  (`/Engine/EditorBlueprintResources/StandardMacros.IsValid` _output
    (:`Is Valid`
      (`self.K2_DestroyActor` _output))))

(event `/Game/Blueprints/Core/Interfaces/BPI_RoundBasedActors.BallBought`
  (params (`Ball Index` :type Integer))
  (bind _output (`|GetArrayItem` (`self.SpawnedBalls`) `Ball Index`))
  (`/Engine/EditorBlueprintResources/StandardMacros.IsValid` _output
    (:`Is Valid`
      (`self.K2_DestroyActor` _output))))

(fn `UserConstructionScript`
  (`|ExecutionSequence`
    (:`then_0`
      (set `self.ShopBallSlotArray` (`|MakeArray` (`self.BP_BallSlotComponent`) (`self.BP_BallSlotComponent1`) (`self.BP_BallSlotComponent2`))))
    (:`then_1`
      (set `self.ShopItemSlotArray` (`|MakeArray` (`self.BP_ShopSlotComponent`) (`self.BP_ShopSlotComponent1`) (`self.BP_ShopSlotComponent2`))))))