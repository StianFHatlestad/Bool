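; BP_BallSlots is a rack of sixteen slot components that spawns and clears the balls assigned in the game instance.
; LoadBalls spawns each assigned ball class at its slot's transform, applies gameplay attributes plus the slot's color and number, then calls SetParams.
; Spawned balls feed BallUpgradeTarget's show-only actor list.
; UnloadBalls destroys them and clears show-only components; UpdateMoney is an empty stub.
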(event `self.ReceiveBeginPlay`
  (bind _asbp_game_instance (cast `/Game/Blueprints/Core/BP_GameInstance` (`GameplayStatics.GetGameInstance`)))
  (set `self.GameInstance` _asbp_game_instance))

(event `/Game/Blueprints/Core/Interfaces/BPI_RoundBasedActors.LoadBalls`
  ;[1 1 1] Load
  (for (_array_element _array_index) (`/Game/Blueprints/Core/BP_GameInstance.BallAssigments` (`self.GameInstance`))
    (bind _output_get (set `self.SBall` _array_element))
    (bind _output (`|GetArrayItem` (`self.BallSlotArray`) _array_index))
    (bind _returnvalue (`|SpawnActorFromClass` (`.BallClass_22_BF39C1D54109D681211D04AC27E726D3` (break `/Game/Blueprints/Balls/S_GameplayAttributes` _output_get)) (`SceneComponent.K2_GetComponentToWorld` _output) "AlwaysSpawn" "OverrideRootScale" null null))
    (set `self.Ball` _returnvalue)
    (`|ExecutionSequence`
      (:`then_0`
        (set `/Game/Blueprints/Balls/BP_Ball.S_GameplayAttributes` (`self.SBall`) (`self.Ball`))
        (set `/Game/Blueprints/Balls/BP_Ball.BallColor` (`/Game/Blueprints/Core/Slots/BP_BallSlotComponent.BallColor` _output) (`self.Ball`))
        (bind _ballnumber (`/Game/Blueprints/Core/Slots/BP_BallSlotComponent.Ballnumber` _output))
        (if (< _ballnumber 16)
          (set `/Game/Blueprints/Balls/BP_Ball.BallNumber` _ballnumber (`self.Ball`))
          (else
            (set `/Game/Blueprints/Balls/BP_Ball.BallNumber` 8 (`self.Ball`)))))
      (:`then_1`
        (`KismetArrayLibrary.Array_Add` (`self.SpawnedBalls`) (`self.Ball`)))
      (:`then_2`
        (`/Game/Blueprints/Balls/BP_Ball.SetParams` (`self.Ball`)))
      (:`then_3`
        (set `SceneCaptureComponent.ShowOnlyActors` (`self.SpawnedBalls`) (`self.BallUpgradeTarget`))))))

(event `/Game/Blueprints/Core/Interfaces/BPI_RoundBasedActors.UnloadBalls`
  ;[1 1 1] Unload
  (for _array_element (`self.SpawnedBalls`)
    (`/Engine/EditorBlueprintResources/StandardMacros.IsValid` _array_element
      (:`Is Valid`
        (`self.K2_DestroyActor` _array_element))))
  (`KismetArrayLibrary.Array_Clear` (`self.SpawnedBalls`))
  (`SceneCaptureComponent.ClearShowOnlyComponents` (`self.BallUpgradeTarget`)))

(fn `UpdateMoney`
  (params (NewMoney :type Integer))
  (return))

(fn `UserConstructionScript`
  (`|ExecutionSequence`
    (:`then_0`
      (set `self.BallSlotArray` (`|MakeArray` (`self.Ballslot`) (`self.Ballslot1`) (`self.Ballslot2`) (`self.Ballslot3`) (`self.Ballslot4`) (`self.Ballslot5`) (`self.Ballslot6`) (`self.Ballslot7`) (`self.Ballslot8`) (`self.Ballslot9`) (`self.Ballslot10`) (`self.Ballslot11`) (`self.Ballslot12`) (`self.Ballslot13`) (`self.Ballslot14`) (`self.Ballslot15`))))))