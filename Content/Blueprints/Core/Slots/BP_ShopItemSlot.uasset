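; BP_ShopItemSlot is a shop slot actor that displays one spawned item at its own location.
; RollItem destroys any current item, then spawns a new actor of the given item's class at the slot's transform, owned by the slot, and stores it as SpawnedItem.
; BuyItem destroys the stored item if valid and returns that same reference.
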(event `/Game/Blueprints/Core/BPI_Items/BPI_ItemShopInterface.RollItem`
  (params (Item :type "/Game/Blueprints/Items/BP_Item Object Reference"))
  (`self.SpawnedItem`
    (:`then`
      (`self.K2_DestroyActor` (`self.SpawnedItem`)))
    (:`else`
      _))
  (bind _returnvalue (`|SpawnActorFromClass` (`GameplayStatics.GetObjectClass` Item) (`self.GetTransform`) "Undefined" "MultiplyWithRoot" self null))
  (set `self.SpawnedItem` _returnvalue))

(fn `BuyItem`
  (returns (OutItem :type "/Game/Blueprints/Items/BP_Item Object Reference"))
  (bind _spawneditem (`self.SpawnedItem`)
    (:`then`
      (`self.K2_DestroyActor` _spawneditem)
      (return _spawneditem))
    (:`else`)))

(fn `UserConstructionScript`)