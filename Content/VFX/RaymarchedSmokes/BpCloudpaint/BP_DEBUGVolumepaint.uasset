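; Debug tool that paints smoke density into a volume render target, using left mouse to paint, right to erase and Left Shift to clear.
; Each tick, with guides on, it projects a point ahead of itself, tests it against the target mesh's bounds and draws debug shapes.
; A dynamic material stamps a sphere at the last valid point, with strongly negative density for erasing, then a fade material is drawn every tick.
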(event `self.ReceiveBeginPlay`
  (bind _returnvalue (`KismetMaterialLibrary.CreateDynamicMaterialInstance` "/Game/VFX/RaymarchedSmokes/M_VolumePaint.M_VolumePaint"))
  (set `self.DynamicVolInstance` _returnvalue))

(event `Key|LeftMouseButton`
  (params (Key :type "Key Structure"))
  (:`Pressed`
    (set `self.Ispainting` true))
  (:`Released`
    (set `self.Ispainting` false)))

(event `Key|RightMouseButton`
  (params (Key :type "Key Structure"))
  (:`Pressed`
    (set `self.Ispainting` true)
    (set `self.Iserasing` true))
  (:`Released`
    (set `self.Ispainting` false)
    (set `self.Iserasing` false)))

(event `Key|LeftShift` :consume false
  (params (Key :type "Key Structure"))
  (:`Pressed`
    (`self.ResetRT`)))

(event `Key|A` :consume false
  (params (Key :type "Key Structure")))

(event `self.ReceiveTick`
  (params (DeltaSeconds :type "Float (single-precision)"))
  (`|ExecutionSequence`
    (:`then_0`
      (`self.UpdateTraces`))
    (:`then_1`
      (if (`self.Ispainting`)
        (`self.DebugPaintSphere` (`self.Iserasing`))))
    (:`then_2`
      (`self.DebugPaintFade`))))

(event `Key|S` :consume false
  (params (Key :type "Key Structure")))

(event `Key|D` :consume false
  (params (Key :type "Key Structure")))

(fn `DebugPaintFade`
  (bind (_canvas _size _context) (`KismetRenderingLibrary.BeginDrawCanvasToRenderTarget` (`self.RT_Rendertarget`)))
  (`Canvas.K2_DrawMaterial` _canvas "/Game/VFX/RaymarchedSmokes/M_VolumeFade.M_VolumeFade" (0.0 0.0) _size (0.0 0.0) (1.0 1.0) 0.0 (0.5 0.5))
  (`KismetRenderingLibrary.EndDrawCanvasToRenderTarget` _context))

(fn `DebugPaintSphere`
  (params (Erase :type Boolean))
  (bind _dynamicvolinstance (`self.DynamicVolInstance`))
  (bind (_canvas _size _context) (`KismetRenderingLibrary.BeginDrawCanvasToRenderTarget` (`self.RT_Rendertarget`)))
  (`MaterialInstanceDynamic.SetVectorParameterValue` (`self.DynamicVolInstance`) "PaintCenter" (`KismetMathLibrary.Conv_VectorToLinearColor` (`self.LastValidPosition`)))
  (`MaterialInstanceDynamic.SetScalarParameterValue` (`self.DynamicVolInstance`) "Density" (`KismetMathLibrary.SelectFloat` -1000.0 (`self.Density`) (`local.Erase`)))
  (`MaterialInstanceDynamic.SetScalarParameterValue` _dynamicvolinstance "Radius" (/ (`self.PaintRadius`) (.z (`.BoxExtent` (`self.GetActorBounds` (`self.TargetMesh`) false false)))))
  (`Canvas.K2_DrawMaterial` _canvas _dynamicvolinstance (0.0 0.0) _size (0.0 0.0) (1.0 1.0) 0.0 (0.5 0.5))
  (`KismetRenderingLibrary.EndDrawCanvasToRenderTarget` _context))

(fn `ResetRT`
  (`KismetRenderingLibrary.ClearRenderTarget2D` (`self.RT_Rendertarget`)))

(fn `UpdateTraces`
  (bind _targetmesh (`self.TargetMesh`))
  (bind (_origin _boxextent) (`self.GetActorBounds` _targetmesh false false))
  (bind _returnvalue (+ (`self.K2_GetActorLocation`) (* (`self.GetActorForwardVector`) (`self.TraceDistance`))))
  (if (`self.ShowGuides`)
    (`KismetSystemLibrary.DrawDebugBox` (`self.K2_GetActorLocation` _targetmesh) _boxextent (struct :`R` 1.0 :`G` 0.012757 :`B` 0.076309 :`A` 1.0) (`self.K2_GetActorRotation` _targetmesh))
    (bind _output_get (set `self.TraceResult` (`KismetMathLibrary.Box_IsPointInside` (`KismetMathLibrary.MakeBoxWithOrigin` _origin _boxextent) (`KismetMathLibrary.InverseTransformLocation` (`self.GetTransform` _targetmesh) _returnvalue))))
    (if _output_get
      (`KismetSystemLibrary.DrawDebugSphere` _returnvalue (`self.PaintRadius`) 12 (struct :`R` 0.012829 :`G` 0.086307 :`B` 1.0 :`A` 1.0))
      (set `self.LastValidPosition` (/ _returnvalue (.x _boxextent)))
      (else
        (`KismetSystemLibrary.DrawDebugSphere` _returnvalue 10.0 12 (struct :`R` 1.0 :`G` 0.055746 :`A` 1.0))))))

(fn `UserConstructionScript`)